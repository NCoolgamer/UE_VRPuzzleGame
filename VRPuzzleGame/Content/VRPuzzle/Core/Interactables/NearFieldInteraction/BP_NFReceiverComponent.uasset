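; Receiver component for VR near-field interactions that tracks sender actors with accepted IDs while they overlap.
; Begin and end overlap checks query each actor's sender ID, update the current sender list and last accepted ID, then fire dispatchers and report back to the sender.
; Optional tick events fire for senders that request them, either per sender or once for all.
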(event EventBeginPlay
  (if (Variables|Default|GetbIgnoreTickEvents)
    (Components|Tick|SetComponentTickEnabled false)))

(event EventTick
  (params (DeltaSeconds :type Float%20%28single-precision%29))
  (if (Utilities|Array|IsNotEmpty (Variables|Default|GetCurrentSenders))
    (CallFunction|CallTickEvents)))

(fn CheckforValidSenderBeginOverlap
  (params (ActorToCheck :type Actor%20Object%20Reference))
  (bind _id (Class|BPINFSender|GetSenderID(Message) ActorToCheck))
  (bind _output_get (LocalVariables|SetThisSenderID _id))
  (if (Utilities|Array|IsEmpty _output_get)
    ;[1 1 1] Not a sender
    (return)
    (elif (or (Variables|Default|GetbAcceptAllIDs) (Utilities|Array|ContainsItem (Variables|Default|GetAcceptedIDs) (LocalVariables|GetThisSenderID)))
      (Variables|Default|SetLastAcceptedID (LocalVariables|GetThisSenderID))
      (Utilities|Array|Add (Variables|Default|GetCurrentSenders) ActorToCheck)
      (Default|CallOnValidSenderBeginOverlap)
      (Class|BPINFSender|ReportReceiver(Message) ActorToCheck self true)
      (else
        ;[1 1 1] Not a valid ID
        (return)))))

(fn CheckforValidSenderEndOverlap
  (params (ActorToCheck :type Actor%20Object%20Reference))
  (bind _currentsenders (Variables|Default|GetCurrentSenders))
  (bind _id (Class|BPINFSender|GetSenderID(Message) ActorToCheck))
  (bind _output_get (LocalVariables|SetThisSenderID _id))
  (if (Utilities|Array|IsEmpty _output_get)
    ;[1 1 1] Not a sender
    (return)
    (elif (or (Variables|Default|GetbAcceptAllIDs) (Utilities|Array|ContainsItem (Variables|Default|GetAcceptedIDs) (LocalVariables|GetThisSenderID)))
      (Utilities|Array|RemoveItem (Variables|Default|GetCurrentSenders) ActorToCheck)
      ;[1 1 1] Update last accepted ID if it was the ID of the removed sender.
      (if (Utilities|Enum|Equal(Enum) (Variables|Default|GetLastAcceptedID) (LocalVariables|GetThisSenderID))
        (bind _id_2 (Class|BPINFSender|GetSenderID(Message) (Utilities|Array|Get(acopy) _currentsenders (Utilities|Array|LastIndex _currentsenders))))
        (Variables|Default|SetLastAcceptedID _id_2))
      (if true
        (Default|CallOnValidSenderEndOverlap (Utilities|Array|Length (Variables|Default|GetCurrentSenders)))
        (Class|BPINFSender|ReportReceiver(Message) ActorToCheck self true)
        (else
          ;[1 1 1] No such item was present in range
          (return)))
      (else
        ;[1 1 1] Not a valid ID
        (return)))))

(fn CallTickEvents
  (for _array_element (Variables|Default|GetCurrentSenders)
    (bind _bshouldcalltick (Class|BPINFSender|ShouldCallTick(Message) _array_element))
    (if _bshouldcalltick
      (Default|CallOnValidSenderTickOverlap)
      ;[1 1 1] Stop if should do it only once
      (if (Variables|Default|GetbTickOncePerAllSenders)
        (return))))
  (return))

(fn GetLastValidSenderID
  (return (Variables|Default|GetLastAcceptedID)))