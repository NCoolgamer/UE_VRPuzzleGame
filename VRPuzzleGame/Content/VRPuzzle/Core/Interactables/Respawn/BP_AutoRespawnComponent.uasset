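; BP_AutoRespawnComponent is an actor component that respawns a fresh copy of its owning actor when play ends for a configured reason.
; BeginPlay stores the owner's transform, and EndPlay spawns the same class there, nudged clear of collisions if needed, then fires OnRespawnedActorCreated with the new actor.
; DestroyPermanently clears the respawn flag before destroying the owner, so that removal leaves no replacement.
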(event EventEndPlay
  (params (EndPlayReason :type EEndPlayReason%20Enum :default "Destroyed"))
  (if (Variables|Default|GetbShouldRespawn)
    (if (Utilities|Array|ContainsItem (Variables|Default|GetRespawnReasons) EndPlayReason)
      (bind _returnvalue (Game|SpawnActorfromClass (Utilities|GetClass (Components|GetOwner)) (Variables|Default|GetRespawnTransform) "AdjustIfPossibleButAlwaysSpawn" "MultiplyWithRoot" 0 0))
      (Default|CallOnRespawnedActorCreated _returnvalue))))

(event EventBeginPlay
  (CallFunction|RememberRespawnTransform))

(fn RememberRespawnTransform
  (Variables|Default|SetRespawnTransform (Transformation|GetActorTransform (Components|GetOwner)))
  (return))

(fn DestroyPermanently
  (Variables|Default|SetbShouldRespawn false)
  (Actor|DestroyActor (Components|GetOwner)))