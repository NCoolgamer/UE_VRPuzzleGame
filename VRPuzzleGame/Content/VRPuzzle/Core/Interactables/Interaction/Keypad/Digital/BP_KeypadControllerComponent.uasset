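; Actor component that runs a digital keypad in the VR puzzle game, managing typed input, its text display and submission.
; SetupKeypad receives keys and a display, caches Submit keys and binds every key's press event.
; Presses emit a tap at the owner, then, if input is allowed, add or remove characters or submit.
; Length limits cap entry and toggle Submit keys, and valid submissions broadcast OnInputSubmit for external handling.
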(event Custom|HandleKeypadKey
  (params (ActionType :type EKeypadKeyActionType%20Enum :default "NewEnumerator0") (KeyCharacter :type String))
  (bind _returnvalue (Components|GetOwner))
  (CallFunction|EmitTapatLocation _returnvalue (Transformation|GetActorLocation _returnvalue))
  (if (Variables|Default|GetbAllowInput)
    (switch Utilities|FlowControl|Switch|SwitchonEKeypadKeyActionType ActionType
      (:NewEnumerator0
        (CallFunction|TryEnterCharacter KeyCharacter))
      (:NewEnumerator1
        (CallFunction|RemoveLastCharacter))
      (:NewEnumerator2
        (CallFunction|TrySubmit)))))

(event Custom|DEBUG%20Submit%20Current%20Input
  (CallFunction|TrySubmit))

(event EventBeginPlay)

(event EventTick
  (params (DeltaSeconds :type Float%20%28single-precision%29)))

(fn SetupKeypad
  (params (KeysArray :type Array%20of%20WBP%20Keypad%20Key%20Object%20References) (InputText :type Text%20Block%20Object%20Reference))
  (Variables|Default|SetKeypadKeys KeysArray)
  (Variables|Default|SetInputDisplay InputText)
  (for _array_element (Variables|Default|GetKeypadKeys)
    (switch Utilities|FlowControl|Switch|SwitchonEKeypadKeyActionType (Variables|/Game/VRPuzzle/Core/Interactables/Interaction/Keypad/Digital/WBP_KeypadKey.WBP_KeypadKey_C|GetKeypadKeyAction _array_element)
      (:NewEnumerator2
        (Utilities|Array|Add (Variables|Default|GetSubmitKeys) _array_element))))
  (CallFunction|FinishKeypadSetup)
  (return))

(fn SwitchSubmitButtonState
  (LocalVariables|SetbShouldEnable (>= (Utilities|String|Len (Variables|Default|GetCurrentInputValue)) (Variables|Default|GetMinCharactersToSubmit)))
  (for _array_element (Variables|Default|GetSubmitKeys)
    (Default|SetEnabledState _array_element (LocalVariables|GetbShouldEnable)))
  (return))

(fn TryEnterCharacter
  (params (NewCharacter :type String))
  (if (<= (+ (Utilities|String|Len NewCharacter) (Utilities|String|Len (Variables|Default|GetCurrentInputValue))) (Variables|Default|GetMaxInputLength))
    (bind _output_get (Variables|Default|SetCurrentInputValue (Utilities|String|Append (Variables|Default|GetCurrentInputValue) NewCharacter)))
    (Rendering|Components|TextRender|SetText (Variables|Default|GetInputDisplay) (Utilities|Text|ToText(String) _output_get))
    (CallFunction|SwitchSubmitButtonState)
    (return)
    (else
      ;[1 1 1] Can't fit
      (return))))

(fn RemoveLastCharacter
  (if (Utilities|Array|IsEmpty (Variables|Default|GetCurrentInputValue))
    ;[1 1 1] Already empty
    (return)
    (else
      (bind _output_get (Variables|Default|SetCurrentInputValue (Utilities|String|GetSubstring (Variables|Default|GetCurrentInputValue) 0 (- (Utilities|String|Len (Variables|Default|GetCurrentInputValue)) 1))))
      (Rendering|Components|TextRender|SetText (Variables|Default|GetInputDisplay) (Utilities|Text|ToText(String) _output_get))
      (CallFunction|SwitchSubmitButtonState)
      (return))))

(fn TrySubmit
  (if (>= (Utilities|String|Len (Variables|Default|GetCurrentInputValue)) (Variables|Default|GetMinCharactersToSubmit))
    (Development|PrintString (Utilities|String|Append "Submitting keypad input: " (Variables|Default|GetCurrentInputValue)))
    (Default|CallOnInputSubmit (Variables|Default|GetCurrentInputValue))
    (return)
    (else
      ;[1 1 1] Too few characters
      (return))))

(fn ClearInput
  (bind _output_get (Variables|Default|SetCurrentInputValue ""))
  (Rendering|Components|TextRender|SetText (Variables|Default|GetInputDisplay) (Utilities|Text|ToText(String) _output_get))
  (CallFunction|SwitchSubmitButtonState)
  (return))

(fn FinishKeypadSetup
  (for _array_element (Variables|Default|GetKeypadKeys)
    (EventDispatchers|BindEventtoOnKeypadKeyPressed _array_element (EventDispatchers|CreateEvent :!event Custom|HandleKeypadKey))
    ;[1 1 1] Reset input
    (Rendering|Components|TextRender|SetText (Variables|Default|GetInputDisplay) (Utilities|Text|ToText(String) (Variables|Default|GetCurrentInputValue)))
    (CallFunction|SwitchSubmitButtonState))
  (return))