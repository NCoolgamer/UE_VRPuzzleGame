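; BP_KeypadKey is an interactable key for a VR puzzle keypad that displays its own character.
; UpdateKeyWidget pushes the key's character into a WBP_KeypadKeyText widget, running in both the construction script and BeginPlay.
; On BeginPlay it registers the key mesh with its interactable component for highlighting, and it exposes that component through GetInteractableComponent.
; It holds no press or input logic itself.
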(event EventBeginPlay
  (Utilities|Array|Add (Variables|/Game/VRPuzzle/Core/Interactables/Interaction/Generic/BP_InteractableComponent.BP_InteractableComponent_C|GetMeshesToHighlight (Variables|Default|GetBP_InteractableComponent)) (Variables|Default|GetKeypadKey))
  (CallFunction|UpdateKeyWidget))

(event Collision|EventActorBeginOverlap
  (params (OtherActor :type Actor%20Object%20Reference)))

(event EventTick
  (params (DeltaSeconds :type Float%20%28single-precision%29)))

(fn ConstructionScript
  (CallFunction|UpdateKeyWidget))

(fn UpdateKeyWidget
  (bind _aswbp_keypad_key_text (Utilities|Casting|CastToWBP_KeypadKeyText (UserInterface|GetWidget (Variables|Default|GetKeypadCharacterDisplay))))
  (Rendering|Components|TextRender|SetText (Variables|/Game/VRPuzzle/Core/Interactables/Interaction/Keypad/WBP_KeypadKeyText.WBP_KeypadKeyText_C|GetKeypadButtonText _aswbp_keypad_key_text) (Variables|Default|GetKeypadKeyCharacter)))

(fn GetInteractableComponent
  (return (Variables|Default|GetBP_InteractableComponent)))