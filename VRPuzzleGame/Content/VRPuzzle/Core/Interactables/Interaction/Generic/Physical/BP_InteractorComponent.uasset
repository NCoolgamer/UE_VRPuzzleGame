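; Actor component that lets a VR hand hover over and trigger interactables in the puzzle game.
; Each tick it sphere-traces along the assigned sender point's right vector and gets the hit actor's interactable component through a message call.
; Enabled interactables within their own max distance become the hovered target and receive hover state changes; otherwise hover clears.
; TryInteract fires the hovered interactable with the interactor's hand and returns whether it succeeded.
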(event EventBeginPlay)

(event EventTick
  (params (DeltaSeconds :type Float%20%28single-precision%29))
  (CallFunction|TraceforInteractables))

(fn TryInteract
  (bind _currenthoveringinteractable (Variables|Default|GetCurrentHoveringInteractable)
    (:then
      (if (Variables|/Game/VRPuzzle/Core/Interactables/Interaction/Generic/Physical/BP_InteractableComponent.BP_InteractableComponent_C|GetbIsEnabled _currenthoveringinteractable)
        ;[1 1 1] Successful interaction
        (Default|Interact (Variables|Default|GetCurrentHoveringInteractable) (Variables|Interaction|GetInteractorHand))
        (return true)
        (else
          ;[1 1 1] The current interactable is disabled
          (CallFunction|ClearCurrentInteractable)
          (return false))))
    (:else
      ;[1 1 1] Nothing to interact with
      (return false))))

(fn TraceforInteractables
  (bind _interactorsenderpoint (Variables|Default|GetInteractorSenderPoint)
    (:then
      (bind (_outhit _returnvalue) (Collision|SphereTraceByChannel (Transformation|GetWorldLocation _interactorsenderpoint) (+ (Transformation|GetWorldLocation _interactorsenderpoint) (* (Math|Vector|GetRightVector _interactorsenderpoint) (Variables|InteractableTracing|GetMaxInteractionDistance))) (Variables|InteractableTracing|GetInteractionTraceRadius) (Variables|InteractableTracing|GetInteractionTraceChannel) false 0 (Variables|InteractableTracing|GetInteractionTraceDebugMode)))
      (if _returnvalue
        (LocalVariables|SetTraceResults _outhit)
        (bind _interactablecomponent (Class|BPIInteractable|GetInteractableComponent(Message) (.HitActor (Collision|BreakHitResult (LocalVariables|GetTraceResults)))))
        (Utilities|IsValid _interactablecomponent
          (:Is%20Valid
            (bind _output_get (LocalVariables|SetInteractableHit _interactablecomponent))
            (if (Variables|/Game/VRPuzzle/Core/Interactables/Interaction/Generic/Physical/BP_InteractableComponent.BP_InteractableComponent_C|GetbIsEnabled _output_get)
              (if (<= (Math|Vector|Distance(Vector) (.Location (Collision|BreakHitResult (LocalVariables|GetTraceResults))) (Transformation|GetWorldLocation (Variables|Default|GetInteractorSenderPoint))) (Variables|/Game/VRPuzzle/Core/Interactables/Interaction/Generic/Physical/BP_InteractableComponent.BP_InteractableComponent_C|GetMaxInteractionDistance (LocalVariables|GetInteractableHit)))
                (if (== (LocalVariables|GetInteractableHit) (Variables|Default|GetCurrentHoveringInteractable))
                  ;[1 1 1] We've hit the same interactable, do nothing
                  (return)
                  (else
                    ;[1 1 1] Hit a new interactable, switch
                    (CallFunction|SwitchtoNewInteractable (LocalVariables|GetInteractableHit))
                    (return)))
                (else
                  ;[1 1 1] Hit an interactable that is too far away
                  (CallFunction|ClearCurrentInteractable)
                  (return)))
              (else
                ;[1 1 1] Hit a disabled interactable
                (CallFunction|ClearCurrentInteractable)
                (return))))
          (:Is%20Not%20Valid
            ;[1 1 1] Hit a normal object
            (CallFunction|ClearCurrentInteractable)
            (return)))
        (else
          ;[1 1 1] Nothing hit.
          (CallFunction|ClearCurrentInteractable)
          (return))))
    (:else
      (Development|PrintString "Assign the sender point component to the interactor!." true true "(R=1.000000,G=0.084041,B=0.000000,A=1.000000)" 5.0 "InteractorUnassignedError")
      (return))))

(fn ClearCurrentInteractable
  (bind _currenthoveringinteractable (Variables|Default|GetCurrentHoveringInteractable)
    (:then
      (Default|ChangeHoverState _currenthoveringinteractable false)
      (Variables|Default|SetCurrentHoveringInteractable 0)
      (return))
    (:else
      (return))))

(fn SwitchtoNewInteractable
  (params (NewInteractable :type BP%20Interactable%20Component%20Object%20Reference))
  (CallFunction|ClearCurrentInteractable)
  (Default|ChangeHoverState NewInteractable true)
  (Variables|Default|SetCurrentHoveringInteractable NewInteractable)
  (return))

(fn SetSenderPointComponent
  (params (NewSenderPoint :type Primitive%20Component%20Object%20Reference))
  (Variables|Default|SetInteractorSenderPoint NewSenderPoint)
  (return))