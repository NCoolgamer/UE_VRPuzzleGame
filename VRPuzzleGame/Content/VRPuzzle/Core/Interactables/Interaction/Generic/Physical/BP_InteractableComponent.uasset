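; Interactable component for a VR puzzle game that gives its owning actor hover highlighting and an interact response.
; On BeginPlay it can auto-collect the owner's mesh components for highlighting through custom depth and stencil.
; A hover counter handles multiple interactors, triggering highlight and hover calls only as the first arrives or the last leaves.
; When enabled, Interact optionally plays haptics on the interacting hand, fires the interact call and prints a debug message.
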(event EventBeginPlay
  (if (Variables|Highlight|GetbAutoCollectMeshesForHighlight)
    (for _array_element (Actor|GetComponentsByClass (Components|GetOwner) "/Script/Engine.MeshComponent")
      (Utilities|Array|Add (Variables|Highlight|GetMeshesToHighlight) _array_element))))

(event EventTick
  (params (DeltaSeconds :type Float%20%28single-precision%29)))

(fn SetHighlightState
  (params (bShouldHighlight :type Boolean))
  (for _array_element (Variables|Highlight|GetMeshesToHighlight)
    (Rendering|SetRenderCustomDepth _array_element bShouldHighlight)
    (Rendering|SetCustomDepthStencilValue _array_element (Variables|Highlight|GetHighlightStencilValue))
    (return)))

(fn ChangeHoverState
  (params (bIsHovering :type Boolean))
  (LocalVariables|SetPreviousInteractorCount (Variables|Hovering|GetHoveringInteractorsCount))
  (if bIsHovering
    (Variables|Hovering|SetHoveringInteractorsCount (+ (Variables|Hovering|GetHoveringInteractorsCount) 1))
    (if (== (LocalVariables|GetPreviousInteractorCount) 0)
      (CallFunction|SetHighlightState true)
      (Default|CallOnHoverStart)
      (return)
      (else
        ;[1 1 1] Already weve hovering with something else, do nothing
        (return)))
    (else
      (bind _output_get (Variables|Hovering|SetHoveringInteractorsCount (- (Variables|Hovering|GetHoveringInteractorsCount) 1)))
      (if (<= _output_get 0)
        (CallFunction|SetHighlightState false)
        (Default|CallOnHoverEnd)
        (return)
        (else
          ;[1 1 1] Still hovering with something else, do nothing.
          (return))))))

(fn Interact
  (params (InteractorHand :type EControllerHand%20Enum :default "Left"))
  (if (Variables|Interaction|GetbIsEnabled)
    (if (Variables|Haptics|GetbTriggerHapticEffect)
      ;[0.03434 0.03434 0.03434] Play Haptic Effect
      (Class|PlayerController|PlayHapticEffect (Game|GetPlayerController 0) (Variables|Haptics|GetHapticFeedbackEffect) InteractorHand 1.0 false))
    (Default|CallOnInteract)
    (Development|PrintString (Utilities|String|Append "Interacted with: " (Utilities|GetDisplayName (Components|GetOwner))))
    (return)
    (else
      (return))))