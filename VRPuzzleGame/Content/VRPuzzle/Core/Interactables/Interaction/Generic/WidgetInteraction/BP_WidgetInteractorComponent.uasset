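; Actor component for VR world-widget interaction that adds the world-widget input mapping context on BeginPlay.
; Each Tick, it line-traces along both supplied hand origins' right vectors for actors reporting as interactable widgets.
; Only the left hand has hover cleanup, hiding the previous widget's cursor.
; Appears unfinished: cursor updates are unwired, StopInteractingForInteractor is empty, and the left WidgetInteraction reference is set to None.
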(event EventBeginPlay
  ;[1 1 1] Add world widget IMC to the input stack, below menu IMC
  (Input|AddMappingContext (PlayerController|LocalPlayerSubsystems|GetEnhancedInputLocalPlayerSubsystem (Game|GetPlayerController 0)) "/Game/VRPuzzle/Core/Input/IMC_WorldWidgets.IMC_WorldWidgets" 2 "(bIgnoreAllPressedKeysUntilRelease=True,bForceImmediately=False,bNotifyUserSettings=False)"))

(event EventTick
  (params (DeltaSeconds :type Float%20%28single-precision%29))
  (CallFunction|TraceforWidgets))

(fn SetWidgetInteractionReferences
  (bind _returnvalue (Components|GetOwner))
  (bind _returnvalue_2 (Actor|GetComponentsByClass _returnvalue "/Script/UMG.WidgetInteractionComponent"))
  (if (> (Utilities|Array|Length _returnvalue_2) 0) ; Are there any Widget Interaction Components attached to us?
    (bind _output_get (LocalVariables|SetLocalWidgetInteractionComponents _returnvalue_2))
    (for _array_element _output_get ; Get the Pawn's Widget Interaction Components
      (if (== (Variables|/Script/UMG.WidgetInteractionComponent|GetPointerIndex _array_element) 0) ; Pointer Index 0 is assigned to the Left WIC
        (Variables|Default|SetWidgetInteractionRefLeft 0)
        (else
          (Variables|Default|SetWidgetInteractionRefRight _array_element))))
    (return)
    (else
      (Development|PrintString "Warning: No WidgetInteractionComponent was found. Menu interaction will FAIL")
      (return))))

(fn SetSenderPointComponents
  (params (NewSenderPointLeft :type Primitive%20Component%20Object%20Reference) (NewSenderPointRight :type Primitive%20Component%20Object%20Reference))
  (Utilities|FlowControl|Sequence
    (:then_0
      ;[1 1 1] Set provided points
      (Utilities|IsValid NewSenderPointLeft
        (:Is%20Valid
          (Variables|Default|SetInteractorTraceOriginComponentLeft NewSenderPointLeft))))
    (:then_1
      (Utilities|IsValid NewSenderPointRight
        (:Is%20Valid
          (Variables|Default|SetInteractorTraceOriginComponentRight NewSenderPointRight))))
    (:then_2
      (return))))

(fn TraceforWidgets
  (Utilities|FlowControl|Sequence
    (:then_0
      (Utilities|FlowControl|Sequence
        (:then_0
          ;[1 1 1] Trace left hand
          (bind _interactortraceorigincomponentleft (Variables|Default|GetInteractorTraceOriginComponentLeft)
            (:then
              (bind _hitactor (CallFunction|TraceforInteractableWidgetsfromComponent _interactortraceorigincomponentleft))
              (LocalVariables|SetHitLeftWidget _hitactor))
            (:else)))
        (:then_1
          ;[1 1 1] Trace right hand
          (bind _interactortraceorigincomponentright (Variables|Default|GetInteractorTraceOriginComponentRight)
            (:then
              (bind _hitactor_2 (CallFunction|TraceforInteractableWidgetsfromComponent _interactortraceorigincomponentright))
              (LocalVariables|SetHitWidgetRight _hitactor_2))
            (:else)))))
    (:then_1
      (Utilities|IsValid (LocalVariables|GetHitLeftWidget)
        (:Is%20Valid
          (Utilities|IsValid (Variables|Default|GetLastLeftWidget)
            (:Is%20Valid
              (if (not (== (Variables|Default|GetLastLeftWidget) (LocalVariables|GetHitLeftWidget)))
                ;[1 1 1] Clean up since we've hit another
                (CallFunction|CleanUpLeftWidget)
                (Variables|Default|SetLastLeftWidget (LocalVariables|GetHitLeftWidget))))))
        (:Is%20Not%20Valid
          ;[1 1 1] Clear left widget since we've didn't hit a widget.
          (CallFunction|CleanUpLeftWidget))))
    (:then_2
      (return (LocalVariables|GetHitLeftWidget) (LocalVariables|GetHitWidgetRight)))))

(fn TraceforInteractableWidgetsfromComponent
  (params (OriginComponent :type Primitive%20Component%20Object%20Reference))
  (bind _returnvalue (Transformation|GetWorldLocation OriginComponent))
  ;[1 1 1] Trace for left hand
  (bind (_outhit _returnvalue_2) (Collision|LineTraceByChannel _returnvalue (+ _returnvalue (* (Math|Vector|GetRightVector OriginComponent) (Variables|Default|GetMaxInteractionRange))) (Variables|Default|GetWidgetTraceChannel) false 0 "ForOneFrame"))
  ;[1 1 1] Check that we've hit an interactable widget, and if so, remember it.
  (if _returnvalue_2
    (bind _bcanbeinteractedwith (Class|BPIInteractableWidget|IsInteractableWidget(Message) (.HitActor (Collision|BreakHitResult _outhit))))
    (if _bcanbeinteractedwith
      (return (.HitActor (Collision|BreakHitResult _outhit)))
      (else
        (return 0) ; Hit something inactive
      ))
    (else
      (return 0) ; Nothing hit
    )))

(fn SendCursorLocation
  (params (WidgetInteraction :type Widget%20Interaction%20Component%20Object%20Reference) (WidgetToSendTo :type Actor%20Object%20Reference))
  (Class|BPIInteractableWidget|UpdateCursorLocation(Message) WidgetToSendTo (.impactpoint (Class|WidgetInteractionComponent|GetLastHitResult WidgetInteraction)))
  (return))

(fn CleanUpLeftWidget
  (Utilities|IsValid (Variables|Default|GetLastLeftWidget)
    (:Is%20Valid
      (Class|BPIInteractableWidget|SetCursorDisplayState(Message) (Variables|Default|GetLastLeftWidget) false)
      (Variables|Default|SetLastLeftWidget 0))))

(fn StopInteractingforInteractor
  (params (WidgetInteractor :type Widget%20Interaction%20Component%20Object%20Reference)))