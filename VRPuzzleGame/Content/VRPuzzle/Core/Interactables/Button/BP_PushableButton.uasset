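; Physical VR push button that fires pressed and held events when overlapping components push it down far enough.
; While pushers overlap, a box trace from below sets the button's depth along its up axis; otherwise MoveComponentTo eases it back.
; Marker components define activation and reset depths, giving hysteresis so each press fires once.
; A press plays haptics on any pushing controller hand, and a debug print is bound at BeginPlay.
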(event OnComponentBeginOverlap(ButtonCollision)
  (params (OverlappedComponent :type Primitive%20Component%20Object%20Reference) (OtherActor :type Actor%20Object%20Reference) (OtherComp :type Primitive%20Component%20Object%20Reference) (OtherBodyIndex :type Integer) (bFromSweep :type Boolean) (SweepResult :type Hit%20Result%20Structure%20%28by%20ref%29))
  ;[1 1 1] Add new pusher
  (if (not (Utilities|Set|Contains (Variables|Default|GetPushers) OtherComp))
    (Utilities|Set|Add (Variables|Default|GetPushers) OtherComp)))

(event OnComponentEndOverlap(ButtonCollision)
  (params (OverlappedComponent :type Primitive%20Component%20Object%20Reference) (OtherActor :type Actor%20Object%20Reference) (OtherComp :type Primitive%20Component%20Object%20Reference) (OtherBodyIndex :type Integer))
  ;[1 1 1] Reset button
  (Utilities|Set|Remove (Variables|Default|GetPushers) OtherComp))

(event Custom|DEBUG_ButtonPressed
  (Development|PrintString "Button Pressed!"))

(event EventBeginPlay
  (CallFunction|RecalculateStartOffsets)
  (EventDispatchers|BindEventtoOnButtonPressed (delegate Custom|DEBUG_ButtonPressed)))

(event EventTick
  (params (DeltaSeconds :type Float%20%28single-precision%29))
  ;[1 1 1] Get push position if colliding
  (if (Utilities|Set|IsNotEmpty (Variables|Default|GetPushers))
    (bind _pushamount (CallFunction|GetPressedButtonPosition))
    (CallFunction|CheckButtonPressed _pushamount)
    ;[1 1 1] Reset if not pushing
    (if (<= _pushamount (Variables|Default|GetResetPushTolerance))
      (Variables|Activation|SetbCanTrigger true))
    (Utilities|FlowControl|Sequence ; Stop resetting the button, then push it
      (:then_0
        (goto _label Stop))
      (:then_1
        (Transformation|SetWorldLocation (Variables|Default|GetButton) (+ (* (Math|Vector|GetUpVector (Variables|Default|GetButton)) (* _pushamount -1.0)) (Variables|Default|GetButtonStartPositionWorld)) false false)))
    (else
      (Utilities|FlowControl|Sequence
        (:then_0
          ;[1 1 1] Return the button to original location if unpressed
          (Components|MoveComponentTo (Variables|Default|GetButton) (Variables|Default|GetButtonStartPositionLocal) "0, 0, 0" false false 0.1 false :!label _label))
        (:then_1
          ;[1 1 1] Reset if moved to neutral position
          (if (<= (* (Class|KismetMathLibrary|GetMinElement (Math|Vector|ProjectVectorontoVector (- (Transformation|GetWorldLocation (Variables|Default|GetButton)) (Variables|Default|GetButtonStartPositionWorld)) (Math|Vector|GetUpVector (Variables|Default|GetButton)))) -1.0) (Variables|Default|GetResetPushTolerance))
            (Variables|Activation|SetbCanTrigger true)))))))

(fn ConstructionScript)

(fn GetPressedButtonPosition
  (bind (_outhit _returnvalue) (Collision|BoxTraceByChannel (Transformation|GetWorldLocation (Variables|Default|GetButtonTraceBottom)) (+ (* (Math|Vector|GetUpVector (Variables|Default|GetButton)) "10.000000,10.000000,10.000000") (Transformation|GetWorldLocation (Variables|Default|GetButtonTraceBottom))) "5.000000,5.000000,0.010000" (Transformation|GetWorldRotation (Variables|Default|GetDefaultSceneRoot)) "TraceTypeQuery4" false 0 "ForOneFrame"))
  (if _returnvalue
    (return (Math|Float|Min(Float) (Variables|Activation|GetActivationPushAmount) (* (Class|KismetMathLibrary|GetMinElement (Utilities|Operators|Subtract (.Location (Collision|BreakHitResult _outhit)) (Variables|Activation|GetButtonTopOffset) (Variables|Default|GetButtonStartPositionWorld))) -1.0)))
    (else
      (return 0.0))))

(fn CheckButtonPressed
  (params (PushAmount :type Float%20%28double-precision%29))
  (if (>= PushAmount (Variables|Activation|GetActivationPushAmount))
    (CallFunction|PressButton)
    (return)
    (else
      (return))))

(fn PressButton
  (Default|CallOnButtonHeldTick)
  (if (Variables|Activation|GetbCanTrigger)
    (Utilities|FlowControl|Sequence
      (:then_0
        ;[1 1 1] Run events
        (Default|CallOnButtonPressed)
        (Variables|Activation|SetbCanTrigger false))
      (:then_1
        (bind _result (Utilities|Set|ToArray (Variables|Default|GetPushers)))
        (for _array_element _result
          (Utilities|IsValid (Components|GetOwner _array_element)
            (:Is%20Valid
              (bind (_biscontroller _hand) (Class|BPITryGetHandSide|TryGetControllerHand(Message) (Components|GetOwner _array_element) _array_element))
              (if _biscontroller
                ;[0.03434 0.03434 0.03434] Play Haptic Effect
                (Class|PlayerController|PlayHapticEffect (Game|GetPlayerController 0) "/Game/VRPuzzle/Core/Interactables/Button/HE_ButtonPress.HE_ButtonPress" _hand 1.0 false)))))))
    (else
      (return))))

(fn RecalculateStartOffsets
  ;[1 1 1] Get offset from the button mesh to the top of the button
  (Variables|Activation|SetButtonTopOffset (- (Transformation|GetWorldLocation (Variables|Default|GetButtonTop)) (Transformation|GetWorldLocation (Variables|Default|GetButton))))
  ;[1 1 1] Remember button initial location
  (Variables|Default|SetButtonStartPositionWorld (Transformation|GetWorldLocation (Variables|Default|GetButton)))
  (Variables|Default|SetButtonStartPositionLocal (Variables|/Script/Engine.SceneComponent|GetRelativeLocation (Variables|Default|GetButton)))
  ;[1 1 1] Calculate push amount needed to trigger the button
  (Variables|Activation|SetActivationPushAmount (Math|Vector|GetMaxElement (Math|Vector|ProjectVectorontoVector (- (Transformation|GetWorldLocation (Variables|Default|GetButtonTop)) (Transformation|GetWorldLocation (Variables|Default|GetButtonActivationHeight))) (Math|Vector|GetUpVector (Variables|Default|GetButton)))))
  ;[1 1 1] Calculate push amount needed to reset the button
  (Variables|Default|SetResetPushTolerance (Math|Vector|GetMaxElement (Math|Vector|ProjectVectorontoVector (- (Transformation|GetWorldLocation (Variables|Default|GetButtonTop)) (Transformation|GetWorldLocation (Variables|Default|GetButtonResetHeight))) (Math|Vector|GetUpVector (Variables|Default|GetButton))))))