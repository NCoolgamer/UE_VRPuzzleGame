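; Actor component that lets a VR puzzle item snap into a holder's hold point and be released again.
; ProcessReceiverReport records the receiver's owner as the candidate holder while in range and holdable.
; TryBeginHold gets the hold point from that holder by interface message, attaches the item and disables physics; EndHold detaches and restores it.
; An optional flag makes Tick retry the hold until it succeeds.
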(event EventBeginPlay)

(event EventTick
  (params (DeltaSeconds :type Float%20%28single-precision%29))
  (if (Variables|Default|GetbTryToHoldUntilHeld)
    (if (Variables|Default|GetbIsHeld)
      (Variables|Default|SetbTryToHoldUntilHeld false)
      (else
        (bind _bheld (CallFunction|TryBeginHold))
        (if _bheld
          (Variables|Default|SetbTryToHoldUntilHeld false))))))

(fn ProcessReceiverReport
  (params (ReceiverComponent :type BP%20NF%20Receiver%20Component%20Object%20Reference) (bIsInRange :type Boolean))
  (if (Variables|Default|GetbCanBeHeld)
    (if bIsInRange
      (Variables|Default|SetHolderActor (Components|GetOwner ReceiverComponent))
      (return)
      (else
        ;[1 1 1] Not in range
        (Variables|Default|SetHolderActor 0)
        (return)))
    (else
      ;[1 1 1] Can't be held
      (Variables|Default|SetHolderActor 0)
      (return))))

(fn TryBeginHold
  (if (Variables|Default|GetbCanBeHeld)
    (bind _holderactor (Variables|Default|GetHolderActor)
      (:then
        (bind _lockpointcomponent (Class|BPIItemHolder|GetHoldPointComponent(Message) _holderactor))
        (Utilities|IsValid _lockpointcomponent
          (:Is%20Valid
            (Variables|Default|SetLockPointComponent _lockpointcomponent)
            (Variables|Default|SetbIsHeld true)
            (Transformation|AttachComponentToComponent (Components|GetOwner) (Variables|Default|GetLockPointComponent) "None" "SnapToTarget" "SnapToTarget" "KeepRelative" true)
            ;[1 1 1] Disable physics
            (bind _itemphysicscomponent (Variables|Default|GetItemPhysicsComponent)
              (:then
                (Physics|SetSimulatePhysics _itemphysicscomponent false)
                (return true))
              (:else
                (Development|PrintString "HoldableItemComponent->ItemPhysicsComponent not set!" true true "(R=1.000000,G=0.000000,B=0.000000,A=1.000000)")
                (return false))))
          (:Is%20Not%20Valid
            ;[1 1 1] No valid lock point configured
            (Development|PrintString "Warning: No valid lock point available to hold the item.")
            (return false))))
      (:else
        ;[1 1 1] Not near holder
        (return false)))
    (else
      ;[1 1 1] Can't be held
      (return false))))

(fn EndHold
  (if (Variables|Default|GetbIsHeld)
    (Variables|Default|GetLockPointComponent
      (:then
        (Transformation|DetachFromActor (Components|GetOwner) "KeepRelative" "KeepRelative" "KeepRelative")
        (Variables|Default|SetbIsHeld false)
        (Variables|Default|SetHolderActor 0)
        ;[1 1 1] Enable physics
        (bind _itemphysicscomponent (Variables|Default|GetItemPhysicsComponent)
          (:then
            (Physics|SetSimulatePhysics _itemphysicscomponent true)
            (return))
          (:else
            (Development|PrintString "HoldableItemComponent->ItemPhysicsComponent not set!" true true "(R=1.000000,G=0.000000,B=0.000000,A=1.000000)")
            (return))))
      (:else
        ;[1 1 1] Lock point invalid
        (return)))
    (else
      ;[1 1 1] Not being held
      (return))))