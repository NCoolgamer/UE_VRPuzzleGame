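; BP_KeycardReader is a VR puzzle keycard reader whose LED changes color when a valid keycard or other sender is in range.
; A Cube collision volume forwards overlap begin and end events to the BP_NFReceiver component, which validates senders.
; The receiver's events set the LEDColor parameter on a dynamic material created at BeginPlay, switching to the disabled color only when no valid senders remain.
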(event OnValidSenderBeginOverlap(BP_NFReceiver)
  (Rendering|Material|SetVectorParameterValue (Variables|Default|GetKeycardLEDMaterial) "LEDColor" (Variables|Default|GetEnabledColor) :!class /Script/Engine.MaterialInstanceDynamic))

(event OnValidSenderEndOverlap(BP_NFReceiver)
  (params (ValidSendersLeft :type Integer))
  (if (<= ValidSendersLeft 0)
    (Rendering|Material|SetVectorParameterValue (Variables|Default|GetKeycardLEDMaterial) "LEDColor" (Variables|Default|GetDisabledColor) :!class /Script/Engine.MaterialInstanceDynamic)))

(event OnValidSenderTickOverlap(BP_NFReceiver))

(event OnComponentBeginOverlap(Cube)
  (params (OverlappedComponent :type Primitive%20Component%20Object%20Reference) (OtherActor :type Actor%20Object%20Reference) (OtherComp :type Primitive%20Component%20Object%20Reference) (OtherBodyIndex :type Integer) (bFromSweep :type Boolean) (SweepResult :type Hit%20Result%20Structure%20%28by%20ref%29))
  (Default|CheckforValidSenderBeginOverlap (Variables|Default|GetBP_NFReceiver) OtherActor))

(event OnComponentEndOverlap(Cube)
  (params (OverlappedComponent :type Primitive%20Component%20Object%20Reference) (OtherActor :type Actor%20Object%20Reference) (OtherComp :type Primitive%20Component%20Object%20Reference) (OtherBodyIndex :type Integer))
  (Default|CheckforValidSenderEndOverlap (Variables|Default|GetBP_NFReceiver) OtherActor))

(event EventBeginPlay
  (bind _returnvalue (Rendering|Material|CreateDynamicMaterialInstance (Variables|Default|GetS_KeycardReader) 2 "/Game/VRPuzzle/Core/Interactables/Keycard/M_KeycardReaderLED.M_KeycardReaderLED" "None" :!class /Script/Engine.PrimitiveComponent))
  (Variables|Default|SetKeycardLEDMaterial _returnvalue))

(event Collision|EventActorBeginOverlap
  (params (OtherActor :type Actor%20Object%20Reference)))

(event EventTick
  (params (DeltaSeconds :type Float%20%28single-precision%29)))

(fn ConstructionScript)