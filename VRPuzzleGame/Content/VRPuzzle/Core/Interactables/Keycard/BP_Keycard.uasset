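; BP_Keycard is a colored keycard interactable for the VR puzzle game that carries a sender ID, exposed through GetSenderID.
; A dynamic material instance tints the card mesh with KeycardColor, applied in the construction script and at BeginPlay.
; When the auto-respawn component creates a replacement, the card copies its ID and color to it and refreshes the material.
; ShouldCallTick returns false.
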(event OnRespawnedActorCreated(BP_AutoRespawnComponent)
  (params (RespawnedActor :type Actor%20Object%20Reference))
  (bind _asbp_keycard (Utilities|Casting|CastToBP_Keycard RespawnedActor))
  (Variables|BP_Keycard_C|SetNFSenderID _asbp_keycard (Variables|Default|GetNFSenderID))
  (Variables|BP_Keycard_C|SetKeycardColor _asbp_keycard (Variables|Default|GetKeycardColor))
  (CallFunction|UpdateBaseColor _asbp_keycard))

(event EventBeginPlay
  (CallFunction|UpdateBaseColor))

(event Collision|EventActorBeginOverlap
  (params (OtherActor :type Actor%20Object%20Reference)))

(event EventTick
  (params (DeltaSeconds :type Float%20%28single-precision%29)))

(fn ConstructionScript
  (CallFunction|UpdateBaseColor))

(fn UpdateBaseColor
  (bind _returnvalue (Rendering|Material|CreateDynamicMaterialInstance (Variables|Default|GetS_Keycard) 0 0 "None" :!class /Script/Engine.PrimitiveComponent))
  (Rendering|Material|SetVectorParameterValue _returnvalue "KeycardColor" (Variables|Default|GetKeycardColor) :!class /Script/Engine.MaterialInstanceDynamic)
  (Rendering|Material|SetMaterial (Variables|Default|GetS_Keycard) 0 _returnvalue))

(fn GetSenderID
  (return (Variables|Default|GetNFSenderID)))

(fn ShouldCallTick
  (return false))