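; BP_CameraCapturerComponent is a component that drives a scene capture into a render target for in-game camera views.
; SetupCamera stores the scene capture component and assigns its texture target.
; StartCapturing triggers CaptureView, which captures on demand and re-arms a one-shot timer using TimeBetweenFrames to throttle updates, until StopCapturing clears it.
; DrawMaterialToRenderTarget can paint a material onto that same target.
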(event EventBeginPlay)

(event EventTick
  (params (DeltaSeconds :type Float%20%28single-precision%29)))

(fn CaptureView
  (Rendering|SceneCapture|CaptureScene (Variables|Default|GetCameraCapturer) :!class /Script/Engine.SceneCaptureComponent2D)
  (bind _returnvalue (Utilities|Time|SetTimerbyEvent (EventDispatchers|CreateEvent :!event CaptureView) (Variables|Default|GetTimeBetweenFrames)))
  (Variables|Default|SetCaptureTimerHandle _returnvalue)
  (return))

(fn StartCapturing
  (Variables|Default|SetbIsCapturing true)
  (CallFunction|CaptureView)
  (return))

(fn StopCapturing
  (bind _capturetimerhandle (Variables|Default|GetCaptureTimerHandle))
  (Variables|Default|SetbIsCapturing false)
  (if (Utilities|Time|IsValidTimerHandle _capturetimerhandle)
    (Utilities|Time|ClearandInvalidateTimerbyHandle _capturetimerhandle)
    (return)
    (else
      (return))))

(fn SetupCamera
  (params (SceneCaptureComponent :type Scene%20Capture%20Component%202D%20Object%20Reference) (CameraTextureTarget :type Texture%20Render%20Target%202D%20Object%20Reference))
  (Variables|Default|SetCameraCapturer SceneCaptureComponent)
  (Variables|/Script/Engine.SceneCaptureComponent2D|SetTextureTarget (Variables|Default|GetCameraCapturer) CameraTextureTarget)
  (return))

(fn DrawMaterialtoRenderTarget
  (params (Material :type Material%20Object%20Reference))
  (Rendering|DrawMaterialtoRenderTarget (Variables|/Script/Engine.SceneCaptureComponent2D|GetTextureTarget (Variables|Default|GetCameraCapturer)) Material)
  (return))