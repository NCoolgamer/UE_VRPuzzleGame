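; VR puzzle component that constrains a grabbed object's movement to a spline.
; A one-time setup call stores the spline and grab component and binds to its grab and drop events.
; While ticking is enabled, it snaps itself and the grab component to the spline point closest to the motion controller plus the initial grab offset.
; Each tick it broadcasts OnMovedByHolding with the spline time at that point.
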(event Custom|StartMovingAlongSpline
  ;[1 1 1] Only tick if grabbed.
  (Components|Tick|SetComponentTickEnabled true)
  (Variables|Default|SetOffset (- (Transformation|GetWorldLocation) (Transformation|GetWorldLocation (Variables|/Game/VRPuzzle/Core/Grabbing/GrabComponent.GrabComponent_C|GetMotionControllerRef (Variables|Default|GetGrabComponent))))))

(event Custom|StopMovingAlongSpline
  ;[1 1 1] Only tick if grabbed.
  (Components|Tick|SetComponentTickEnabled false))

(event EventTick
  (params (DeltaSeconds :type Float%20%28single-precision%29))
  (bind _grabcomponent (Variables|Default|GetGrabComponent))
  (bind _offset (Variables|Default|GetOffset))
  (bind _grabbablemovementspline (Variables|Default|GetGrabbableMovementSpline))
  (bind _grabbablemovementspline_2 (Variables|Default|GetGrabbableMovementSpline))
  (bind _motioncontrollerref (Variables|/Game/VRPuzzle/Core/Grabbing/GrabComponent.GrabComponent_C|GetMotionControllerRef _grabcomponent))
  (bind _returnvalue (Transformation|GetWorldLocation _motioncontrollerref))
  (bind _returnvalue_2 (+ _returnvalue _offset))
  (bind _returnvalue_3 (Spline|FindLocationClosesttoWorldLocation _grabbablemovementspline _returnvalue_2 "World"))
  (Transformation|SetWorldLocation _returnvalue_3 false false)
  (Transformation|SetWorldLocation (Variables|Default|GetGrabComponent) _returnvalue_3 false false) ; Also lock the grab component to the spline
  (Default|CallOnMovedbyHolding (Class|SplineComponent|GetTimeatDistanceAlongSpline _grabbablemovementspline_2 (Class|SplineComponent|GetDistanceAlongSplineatLocation _grabbablemovementspline_2 _returnvalue_3 "World"))))

(fn SetupLockedGrabbable
  (params (MovementSpline :type Spline%20Component%20Object%20Reference) (GrabComponent :type Grab%20Component%20Object%20Reference))
  (Variables|Default|GetGrabComponent
    (:then
      (Development|PrintString "Error: Trying to setup the same locked grabbable more than once.")
      (return))
    (:else
      (Variables|Default|SetGrabbableMovementSpline MovementSpline)
      (bind _output_get (Variables|Default|SetGrabComponent GrabComponent))
      ;[1 1 1] Bind to grab events
      (EventDispatchers|BindEventtoOnGrabbed _output_get (EventDispatchers|CreateEvent :!event Custom|StartMovingAlongSpline))
      (EventDispatchers|BindEventtoOnDropped _output_get (EventDispatchers|CreateEvent :!event Custom|StopMovingAlongSpline)))))

(fn GetClosestPointonSpline
  (params (PointToCheck :type Vector))
  (bind _grabbablemovementspline (Variables|Default|GetGrabbableMovementSpline))
  (bind _grabbablemovementspline_2 (Variables|Default|GetGrabbableMovementSpline))
  (bind _returnvalue (Class|SplineComponent|FindInputKeyClosesttoWorldLocation _grabbablemovementspline_2 PointToCheck))
  (bind _returnvalue_2 (Math|Float|Floor _returnvalue))
  (bind _returnvalue_3 (+ _returnvalue_2 1))
  (return (Spline|GetLocationatDistanceAlongSpline (Variables|Default|GetGrabbableMovementSpline) (* (- (Spline|GetDistanceAlongSplineatSplinePoint _grabbablemovementspline _returnvalue_2) (Spline|GetDistanceAlongSplineatSplinePoint _grabbablemovementspline _returnvalue_3)) (- _returnvalue (Math|Conversions|ToFloat(Integer) _returnvalue_3))) "World")))