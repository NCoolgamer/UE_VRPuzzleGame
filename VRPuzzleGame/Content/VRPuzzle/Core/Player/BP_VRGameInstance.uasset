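; Game instance for the VR puzzle game that owns the station save data, level transitions and level record timing.
; On init it loads the save slot or creates a fresh save object, then fires a reload notification, as does deleting the save.
; Loading a level by ID unlocks that sector, saves and opens the mapped level.
; A timer saves each level's time only when it sets a new record.
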(event Custom|StartLoadingLevel
  (params (LevelID :type String%20%28by%20ref%29))
  (bind _levelstoload (Variables|Default|GetLevelsToLoad))
  (bind (_value _returnvalue) (Utilities|Map|Find _levelstoload LevelID))
  ;[0.7052 0.8427 1] Load new level by ID
  (if _returnvalue
    ;;[1 1 1] Add new sector to available sectors
    (Utilities|Array|AddUnique (Variables|/Game/VRPuzzle/Core/Saving/BP_StationGameSave.BP_StationGameSave_C|GetAvailableSectors (Variables|Default|GetSaveGameInstance)) LevelID)
    (CallFunction|SaveGame)
    (Game|OpenLevel(byName) _value)
    (else
      (Development|PrintString (Utilities|String|Append "Error: Failed to find level with ID: " LevelID)))))

(event Custom|SaveGame
  (bind _savegameinstance (Variables|Default|GetSaveGameInstance))
  ;[0.05057 1 0] Save game to slot
  (Utilities|IsValid (Variables|Default|GetSaveGameInstance)
    (:Is%20Valid
      _)
    (:Is%20Not%20Valid
      (CallFunction|TryLoadingSave)))
  (SaveGame|SaveGametoSlot _savegameinstance (Variables|/Game/VRPuzzle/Core/Saving/BP_StationGameSave.BP_StationGameSave_C|GetSaveSlotName _savegameinstance) (Variables|/Game/VRPuzzle/Core/Saving/BP_StationGameSave.BP_StationGameSave_C|GetSaveUserIndex _savegameinstance)))

(event Custom|DeleteSaveData
  (bind _savegameinstance (Variables|Default|GetSaveGameInstance))
  ;[1 0 0] Delete the savegame
  (SaveGame|DeleteGameinSlot (Variables|/Game/VRPuzzle/Core/Saving/BP_StationGameSave.BP_StationGameSave_C|GetSaveSlotName _savegameinstance) (Variables|/Game/VRPuzzle/Core/Saving/BP_StationGameSave.BP_StationGameSave_C|GetSaveUserIndex _savegameinstance))
  (CallFunction|TryLoadingSave))

(event Custom|StartLevelTimer
  (Variables|Default|SetStartTime (Utilities|Time|GetGameTimeinSeconds)))

(event EventInit
  ;[1 1 1] Try loading on init play
  (CallFunction|TryLoadingSave))

(fn TryLoadingSave
  (bind _returnvalue (SaveGame|CreateSaveGameObject "/Game/VRPuzzle/Core/Saving/BP_StationGameSave.BP_StationGameSave_C"))
  (bind _returnvalue_2 (SaveGame|LoadGamefromSlot (Variables|/Game/VRPuzzle/Core/Saving/BP_StationGameSave.BP_StationGameSave_C|GetSaveSlotName _returnvalue) (Variables|/Game/VRPuzzle/Core/Saving/BP_StationGameSave.BP_StationGameSave_C|GetSaveUserIndex _returnvalue)))
  (bind _asbp_station_game_save (Utilities|Casting|CastToBP_StationGameSave _returnvalue_2)
    (:then
      (Variables|Default|SetSaveGameInstance _asbp_station_game_save)
      (Default|CallOnSaveDataReload)
      (return))
    (:CastFailed
      (Variables|Default|SetSaveGameInstance _returnvalue)
      (Default|CallOnSaveDataReload)
      (return))))

(fn StopandSaveLevelTimer
  (params (LevelId :type String%20%28by%20ref%29))
  (bind _savegameinstance (Variables|Default|GetSaveGameInstance))
  (bind _recordtimes (Variables|/Game/VRPuzzle/Core/Saving/BP_StationGameSave.BP_StationGameSave_C|GetRecordTimes _savegameinstance))
  (bind (_value _returnvalue) (Utilities|Map|Find _recordtimes LevelId))
  (LocalVariables|SetElapsedTime (- (Utilities|Time|GetGameTimeinSeconds) (Variables|Default|GetStartTime)))
  (if (or (not _returnvalue) (< (LocalVariables|GetElapsedTime) _value))
    ;[1 1 1] Overwrite time
    (Utilities|Map|Add (Variables|/Game/VRPuzzle/Core/Saving/BP_StationGameSave.BP_StationGameSave_C|GetRecordTimes (Variables|Default|GetSaveGameInstance)) LevelId (LocalVariables|GetElapsedTime))
    (CallFunction|SaveGame)))