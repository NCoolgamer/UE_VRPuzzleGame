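; VR grabbable repair gun that toggles a Niagara weld effect while a shoot input is held.
; Grabbing adds a hand-specific input mapping context, and dropping stops welding and removes it; both shoot inputs check for the left hand.
; A holdable-item component processes receiver reports, releases its hold on grab attempts and seeks a new hold on drop.
; It exposes its item ID as sender and the welding state as its tick condition.
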(event OnGrabbed(GrabComponentSnap)
  ;[1 1 1] Add IMC for shooting when grabbed, and remove it when dropped.
  (Input|EnableInput (Game|GetPlayerController 0))
  (Input|AddMappingContext (PlayerController|LocalPlayerSubsystems|GetEnhancedInputLocalPlayerSubsystem (Game|GetPlayerController 0)) (select (Utilities|Enum|Equal(Enum) (Default|GetHeldbyHand (Variables|Default|GetGrabComponentSnap)) "Right") "/Game/VRPuzzle/Core/Input/IMC_Weapon_Right.IMC_Weapon_Right" "/Game/VRPuzzle/Core/Input/IMC_Weapon_Left.IMC_Weapon_Left") 2 "(bIgnoreAllPressedKeysUntilRelease=True,bForceImmediately=False,bNotifyUserSettings=False)")
  (Variables|/Game/VRPuzzle/Core/Interactables/ItemHolder/BP_HoldableItemComponent.BP_HoldableItemComponent_C|SetbCanBeHeld (Variables|Default|GetBP_HoldableItemComponent) false))

(event OnDropped(GrabComponentSnap)
  ;[1 1 1] Add IMC for shooting when grabbed, and remove it when dropped.
  (CallFunction|SetWeldingState false)
  (Input|DisableInput (Game|GetPlayerController 0))
  (Input|RemoveMappingContext (PlayerController|LocalPlayerSubsystems|GetEnhancedInputLocalPlayerSubsystem (Game|GetPlayerController 0)) (select (Utilities|Enum|Equal(Enum) (Default|GetHeldbyHand (Variables|Default|GetGrabComponentSnap)) "Right") "/Game/VRPuzzle/Core/Input/IMC_Weapon_Right.IMC_Weapon_Right" "/Game/VRPuzzle/Core/Input/IMC_Weapon_Left.IMC_Weapon_Left") "(bIgnoreAllPressedKeysUntilRelease=True,bForceImmediately=False,bNotifyUserSettings=False)")
  (Variables|/Game/VRPuzzle/Core/Interactables/ItemHolder/BP_HoldableItemComponent.BP_HoldableItemComponent_C|SetbCanBeHeld (Variables|Default|GetBP_HoldableItemComponent) true)
  (Variables|/Game/VRPuzzle/Core/Interactables/ItemHolder/BP_HoldableItemComponent.BP_HoldableItemComponent_C|SetbTryToHoldUntilHeld (Variables|Default|GetBP_HoldableItemComponent) true))

(event OnTryGrab(GrabComponentSnap)
  (Default|EndHold (Variables|Default|GetBP_HoldableItemComponent)))

(event Input|EnhancedActionEvents|EnhancedInputActionIA_Shoot_Left
  (params (ActionValue :type Boolean) (ElapsedSeconds :type Float%20%28double-precision%29) (TriggeredSeconds :type Float%20%28double-precision%29) (InputAction :type Input%20Action%20Object%20Reference :default "/Game/VRPuzzle/Core/Input/Actions/IA_Shoot_Left.IA_Shoot_Left"))
  ;[1 1 1] Test "shooting"
  (:Started
    (if (CallFunction|CheckHeldbyHand "Left")
      (CallFunction|SetWeldingState true)))
  (:Completed
    (if (CallFunction|CheckHeldbyHand "Left")
      (CallFunction|SetWeldingState false))))

(event Input|EnhancedActionEvents|EnhancedInputActionIA_Shoot_Right
  (params (ActionValue :type Boolean) (ElapsedSeconds :type Float%20%28double-precision%29) (TriggeredSeconds :type Float%20%28double-precision%29) (InputAction :type Input%20Action%20Object%20Reference :default "/Game/VRPuzzle/Core/Input/Actions/IA_Shoot_Right.IA_Shoot_Right"))
  ;[1 1 1] Test "shooting"
  (:Started
    (if (CallFunction|CheckHeldbyHand "Left")
      (CallFunction|SetWeldingState true)))
  (:Completed
    (if (CallFunction|CheckHeldbyHand "Left")
      (CallFunction|SetWeldingState false))))

(event EventBeginPlay
  (Variables|/Game/VRPuzzle/Core/Interactables/ItemHolder/BP_HoldableItemComponent.BP_HoldableItemComponent_C|SetItemPhysicsComponent (Variables|Default|GetBP_HoldableItemComponent) (Variables|Default|GetS_RepairGun))
  (Variables|/Game/VRPuzzle/Core/Interactables/ItemHolder/BP_HoldableItemComponent.BP_HoldableItemComponent_C|SetbTryToHoldUntilHeld (Variables|Default|GetBP_HoldableItemComponent) true))

(event Collision|EventActorBeginOverlap
  (params (OtherActor :type Actor%20Object%20Reference)))

(event EventTick
  (params (DeltaSeconds :type Float%20%28single-precision%29)))

(event EventReportReceiver
  (params (ReceiverComponent :type BP%20NF%20Receiver%20Component%20Object%20Reference) (bInRange :type Boolean))
  (Default|ProcessReceiverReport (Variables|Default|GetBP_HoldableItemComponent) ReceiverComponent bInRange))

(fn ConstructionScript)

(fn CheckHeldbyHand
  (params (Hand :type EControllerHand%20Enum :default "Left"))
  (return (Utilities|Enum|Equal(Enum) (Default|GetHeldbyHand (Variables|Default|GetGrabComponentSnap)) Hand)))

(fn SetWeldingState
  (params (bShouldWeld :type Boolean))
  (Variables|Default|SetShould%20Weld bShouldWeld)
  (Components|Activation|SetActive (Variables|Default|GetNS_Weld) (Variables|Default|GetShould%20Weld) false)
  (return))

(fn GetSenderID
  (return (Variables|Default|GetItemID)))

(fn ShouldCallTick
  (return (Variables|Default|GetShould%20Weld)))