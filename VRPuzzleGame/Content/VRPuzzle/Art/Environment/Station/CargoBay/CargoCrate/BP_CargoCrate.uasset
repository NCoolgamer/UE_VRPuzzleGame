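; Cargo crate prop for the station cargo bay, with a tintable body, numbered labels and front and back double doors.
; Construction and BeginPlay apply the tint through a dynamic material and write the crate number to both widgets, picking a random one if zero.
; OpenDoors and CloseDoors animate each door pair and toggle its collision, disabling interior collision while either side is open.
; A separate function randomizes rotation and picks a palette color.
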(event Custom|DEBUG_CloseAllDoors
  (CallFunction|CloseDoors false)
  (CallFunction|CloseDoors true))

(event Custom|DEBUG_OpenAllDoors
  (CallFunction|OpenDoors false)
  (CallFunction|OpenDoors true))

(event EventBeginPlay
  (CallFunction|SetCrateColorTint)
  (CallFunction|UpdateCrateNumberTexts))

(fn ConstructionScript
  (CallFunction|SetCrateColorTint)
  (CallFunction|UpdateCrateNumberTexts))

(fn SetCrateColorTint
  (bind _returnvalue (Rendering|Material|CreateDynamicMaterialInstance (Variables|Default|GetS_CargoCrate) 0 0 "None" :!class /Script/Engine.PrimitiveComponent))
  (bind _output_get (Variables|Default|SetCrateMaterial _returnvalue))
  (Rendering|Material|SetVectorParameterValue _output_get "CrateTint" (Variables|Default|GetCrateColorTint) :!class /Script/Engine.MaterialInstanceDynamic)
  (Rendering|Material|SetMaterial (Variables|Default|GetS_CargoCrate) 0 (Variables|Default|GetCrateMaterial))
  (return))

(fn RandomizeCrate
  (Transformation|SetActorRotation (Math|Random|RandomRotator true))
  (Variables|Default|SetCrateColorTint (.OutItem (Utilities|Array|Random (Variables|Default|GetPossibleColors)))))

(fn UpdateCrateNumberTexts
  (if (== (Variables|Default|GetCrateNumber) 0)
    (Variables|Default|SetCrateNumber (Math|Random|RandomIntegerinRange 0 999999)))
  (Utilities|FlowControl|Sequence
    (:then_0
      (bind _aswbp_crate_number (Utilities|Casting|CastToWBP_CrateNumber (UserInterface|GetWidget (Variables|Default|GetNumberWidgetR))))
      (Rendering|Components|TextRender|SetText (Variables|/Game/VRPuzzle/Art/Environment/Station/CargoBay/CargoCrate/WBP_CrateNumber.WBP_CrateNumber_C|GetCrateNumberText _aswbp_crate_number) (Utilities|Text|ToText(Integer) (Variables|Default|GetCrateNumber) false false 6 6)))
    (:then_1
      (bind _aswbp_crate_number_2 (Utilities|Casting|CastToWBP_CrateNumber (UserInterface|GetWidget (Variables|Default|GetNumberWidgetL))))
      (Rendering|Components|TextRender|SetText (Variables|/Game/VRPuzzle/Art/Environment/Station/CargoBay/CargoCrate/WBP_CrateNumber.WBP_CrateNumber_C|GetCrateNumberText _aswbp_crate_number_2) (Utilities|Text|ToText(Integer) (Variables|Default|GetCrateNumber) false false 6 6))
      (return))))

(fn OpenDoors
  (params (bOpenBack :type Boolean))
  ;[1 1 1] Check if already open
  (if (not (select bOpenBack (Variables|Default|GetbBackOpen) (Variables|Default|GetbFrontOpen)))
    (for _array_element (select bOpenBack (Utilities|Array|MakeArray (Variables|Default|GetSM_CrateDoor_BackLeft) (Variables|Default|GetSM_CrateDoor_BackRight)) (Utilities|Array|MakeArray (Variables|Default|GetSM_CrateDoor_FrontLeft) (Variables|Default|GetSM_CrateDoor_FrontRight)))
      (Components|Animation|PlayAnimation _array_element "/Game/VRPuzzle/Art/Environment/Station/CargoBay/CargoCrate/AS_OpenDoor.AS_OpenDoor" false)
      (Collision|SetCollisionEnabled (select bOpenBack (Variables|Default|GetDoorCollisionBack) (Variables|Default|GetDoorCollisionFront)) "NoCollision")
      (if bOpenBack
        (Variables|Default|SetbBackOpen true)
        (else
          (Variables|Default|SetbFrontOpen true)))
      (Collision|SetCollisionEnabled (Variables|Default|GetInsideCollision) (select (or (Variables|Default|GetbFrontOpen) (Variables|Default|GetbBackOpen)) "NoCollision" "QueryAndPhysics")))
    (return)
    (else
      (return))))

(fn CloseDoors
  (params (bCloseBack :type Boolean))
  ;[1 1 1] Check if already closed
  (if (select bCloseBack (Variables|Default|GetbBackOpen) (Variables|Default|GetbFrontOpen))
    (for _array_element (select bCloseBack (Utilities|Array|MakeArray (Variables|Default|GetSM_CrateDoor_BackLeft) (Variables|Default|GetSM_CrateDoor_BackRight)) (Utilities|Array|MakeArray (Variables|Default|GetSM_CrateDoor_FrontLeft) (Variables|Default|GetSM_CrateDoor_FrontRight)))
      (Components|Animation|PlayAnimation _array_element "/Game/VRPuzzle/Art/Environment/Station/CargoBay/CargoCrate/AS_CloseDoor.AS_CloseDoor" false)
      (Collision|SetCollisionEnabled (select bCloseBack (Variables|Default|GetDoorCollisionBack) (Variables|Default|GetDoorCollisionFront)) "QueryAndPhysics")
      (if bCloseBack
        (Variables|Default|SetbBackOpen false)
        (else
          (Variables|Default|SetbFrontOpen false)))
      (Collision|SetCollisionEnabled (Variables|Default|GetInsideCollision) (select (or (Variables|Default|GetbFrontOpen) (Variables|Default|GetbBackOpen)) "NoCollision" "QueryAndPhysics")))
    (return)
    (else
      (return))))