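; BP_SecurityCamera is a rotatable security camera for the cargo bay's camera control panel in the VR puzzle game.
; StartCapturing and StopCapturing toggle a throttled scene capture, which uses a re-armed one-shot timer spaced by TimeBetweenFrames instead of Tick.
; Left and right tick events, triggered externally, ease the pivot's yaw toward its bounds at constant speed.
; The construction script and BeginPlay both apply the start rotation.
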(event Custom|CaptureView
  ;[1 1 1] Capture and schedule next
  (Rendering|SceneCapture|CaptureScene (Variables|Default|GetCameraCapturer) :!class /Script/Engine.SceneCaptureComponent2D)
  (bind _returnvalue (Utilities|Time|SetTimerbyEvent (EventDispatchers|CreateEvent :!event Custom|CaptureView) (Variables|Default|GetTimeBetweenFrames)))
  (Variables|Default|SetCaptureTimerHandle _returnvalue))

(event Custom|RotateCameraTick
  (params (bRotateRight :type Boolean))
  (CallFunction|SetCameraRotation (Math|Float|SelectFloat (Math|Interpolation|FInterptoConstant (.yaw (Variables|/Script/Engine.SceneComponent|GetRelativeRotation (Variables|Default|GetCameraRotationPivot))) (.y (Variables|Default|GetRotationBounds)) (Utilities|Time|GetWorldDeltaSeconds) (Variables|Default|GetCameraRotationSpeed)) (Math|Interpolation|FInterptoConstant (.yaw (Variables|/Script/Engine.SceneComponent|GetRelativeRotation (Variables|Default|GetCameraRotationPivot))) (.x (Variables|Default|GetRotationBounds)) (Utilities|Time|GetWorldDeltaSeconds) (Variables|Default|GetCameraRotationSpeed)) bRotateRight)))

(event Custom|RotateCameraRightTick
  (CallFunction|RotateCameraTick true))

(event Custom|RotateCameraLeftTick
  (CallFunction|RotateCameraTick false))

(event EventBeginPlay
  (CallFunction|SetCameraRotation (Variables|Default|GetStartRotation)))

(event Collision|EventActorBeginOverlap
  (params (OtherActor :type Actor%20Object%20Reference)))

(event EventTick
  (params (DeltaSeconds :type Float%20%28single-precision%29)))

(fn ConstructionScript
  (CallFunction|SetCameraRotation (Variables|Default|GetStartRotation)))

(fn StartCapturing
  (Variables|Default|SetbIsCapturing true)
  (CallFunction|CaptureView)
  (return))

(fn StopCapturing
  (bind _capturetimerhandle (Variables|Default|GetCaptureTimerHandle))
  (Variables|Default|SetbIsCapturing false)
  (if (Utilities|Time|IsValidTimerHandle _capturetimerhandle)
    (Utilities|Time|ClearandInvalidateTimerbyHandle _capturetimerhandle)
    (return)
    (else
      (return))))

(fn SetCameraRotation
  (params (NewRotation_Yaw :type Float%20%28single-precision%29))
  (bind _camerarotationpivot (Variables|Default|GetCameraRotationPivot))
  (bind _relativerotation (Variables|/Script/Engine.SceneComponent|GetRelativeRotation _camerarotationpivot))
  (Transformation|SetRelativeRotation (Variables|Default|GetCameraRotationPivot) (Math|Rotator|MakeRotator (.roll _relativerotation) (.pitch _relativerotation) NewRotation_Yaw) false false))