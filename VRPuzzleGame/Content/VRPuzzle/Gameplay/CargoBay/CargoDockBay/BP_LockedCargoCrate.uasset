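; BP_LockedCargoCrate is a cargo crate for the VR puzzle's cargo bay, with front and back doors locked by keypads.
; On BeginPlay it binds to the submit event of each child-actor digital keypad's controller component.
; A submission matching the shared CorrectCode calls OpenDoors for that keypad's side and sets IsOpen.
; Debug events open either side without the code.
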(event Custom|OnKeypadSubmitBack
  (params (InputValue :type String))
  ;[1 1 1] Try to open the door with the password
  (if (Utilities|Enum|Equal(Enum) InputValue (Variables|Default|GetCorrectCode))
    (CallFunction|OpenDoors true)
    (Variables|Default|SetbIsOpen true)))

(event Custom|OnKeypadSubmitFront
  (params (InputValue :type String))
  ;[1 1 1] Try to open the door with the password
  (if (Utilities|Enum|Equal(Enum) InputValue (Variables|Default|GetCorrectCode))
    (CallFunction|OpenDoors false)
    (Variables|Default|SetbIsOpen true)))

(event Custom|DEBUG_OpenBack
  ;[1 1 1] Try to open the door with the password
  (CallFunction|OpenDoors true)
  (Variables|Default|SetbIsOpen true))

(event Custom|DEBUG_OpenFront
  ;[1 1 1] Try to open the door with the password
  (CallFunction|OpenDoors false)
  (Variables|Default|SetbIsOpen true))

(event EventBeginPlay
  ;[1 1 1] Bind to keypads
  (|CallParentFunction)
  (Utilities|FlowControl|Sequence
    (:then_0
      (bind _aswbp_digital_keypad (Utilities|Casting|CastToWBP_DigitalKeypad (Variables|/Script/Engine.ChildActorComponent|GetChildActor (Variables|Default|GetWBP_DigitalKeypadFront))))
      (EventDispatchers|BindEventtoOnInputSubmit (Variables|/Game/VRPuzzle/Core/Interactables/Interaction/Keypad/Digital/WBP_DigitalKeypad.WBP_DigitalKeypad_C|GetBP_KeypadControllerComponent _aswbp_digital_keypad) (EventDispatchers|CreateEvent :!event Custom|OnKeypadSubmitFront)))
    (:then_1
      (bind _aswbp_digital_keypad_2 (Utilities|Casting|CastToWBP_DigitalKeypad (Variables|/Script/Engine.ChildActorComponent|GetChildActor (Variables|Default|GetWBP_DigitalKeypadBack))))
      (EventDispatchers|BindEventtoOnInputSubmit (Variables|/Game/VRPuzzle/Core/Interactables/Interaction/Keypad/Digital/WBP_DigitalKeypad.WBP_DigitalKeypad_C|GetBP_KeypadControllerComponent _aswbp_digital_keypad_2) (EventDispatchers|CreateEvent :!event Custom|OnKeypadSubmitBack)))))

(fn ConstructionScript
  (|CallParentFunction))