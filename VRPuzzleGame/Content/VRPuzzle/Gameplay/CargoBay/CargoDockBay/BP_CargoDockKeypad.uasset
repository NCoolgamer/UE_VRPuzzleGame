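; BP_CargoDockKeypad is an interactable widget-based keypad for the cargo dock bay in a VR puzzle game.
; On BeginPlay it casts its widget to WBP_CargoDockKeypad, caches it, and passes its keys and input display to the keypad controller component.
; ReportDockingProgress forwards the display state and time left to the widget, so the same screen shows docking progress.
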(event EventBeginPlay
  (bind _aswbp_cargo_dock_keypad (Utilities|Casting|CastToWBP_CargoDockKeypad (UserInterface|GetWidget (Variables|Default|GetWidget))))
  (bind _output_get (Variables|Default|SetCargoDockKeypadWidget _aswbp_cargo_dock_keypad))
  (Default|SetupKeypad (Variables|Default|GetBP_KeypadControllerComponent) (Default|GetKeypadKeys _output_get) (Variables|/Game/VRPuzzle/Gameplay/CargoBay/CargoDockBay/WBP_CargoDockKeypad.WBP_CargoDockKeypad_C|GetInputDisplay _output_get)))

(fn ConstructionScript)

(fn ReportDockingProgress
  (params (bDisplayProgress :type Boolean) (TimeLeft :type Float%20%28double-precision%29))
  (Default|ProcessDockingProgress (Variables|Default|GetCargoDockKeypadWidget) bDisplayProgress TimeLeft))

(fn IsInteractableWidget
  (return true))