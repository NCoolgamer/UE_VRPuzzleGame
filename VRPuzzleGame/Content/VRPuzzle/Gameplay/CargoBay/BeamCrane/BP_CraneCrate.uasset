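; BP_CraneCrate is a grabbable, color-tinted crate for the cargo bay beam crane in the VR puzzle game.
; The construction script applies a dynamic MI_CraneCrate material instance tinted by CrateColor.
; Getter functions expose its grab eligibility, extents, grab point component and that point's world-space offset from the crate mesh.
; A SetCollisionStatus event toggles actor collision; the crate runs no other gameplay logic itself.
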(event EventBeginPlay)

(event Collision|EventActorBeginOverlap
  (params (OtherActor :type Actor%20Object%20Reference)))

(event EventTick
  (params (DeltaSeconds :type Float%20%28single-precision%29)))

(event EventSetCollisionStatus
  (params (bShouldCollide :type Boolean))
  (Collision|SetActorEnableCollision bShouldCollide))

(fn ConstructionScript
  (bind _returnvalue (Rendering|Material|CreateDynamicMaterialInstance (Variables|Default|GetCrate) 0 "/Game/VRPuzzle/Gameplay/CargoBay/BeamCrane/MI_CraneCrate.MI_CraneCrate" "None" :!class /Script/Engine.PrimitiveComponent))
  (Rendering|Material|SetVectorParameterValue _returnvalue "Tint" (Variables|Default|GetCrateColor) :!class /Script/Engine.MaterialInstanceDynamic)
  (Rendering|Material|SetMaterial (Variables|Default|GetCrate) 0 _returnvalue))

(fn GetCanbeGrabbed
  (return (Variables|Default|GetbCanBeGrabbed)))

(fn TryGetExtents
  (return (Variables|Default|GetExtents) (- (Transformation|GetWorldLocation (Variables|Default|GetGrabPoint)) (Transformation|GetWorldLocation (Variables|Default|GetCrate)))))

(fn TryGetGrabPointComponent
  (return (Variables|Default|GetGrabPoint)))