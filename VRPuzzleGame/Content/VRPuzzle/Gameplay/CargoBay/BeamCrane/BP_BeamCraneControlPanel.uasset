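; Control panel for the cargo bay beam crane in a VR puzzle, starting broken with a blacked-out camera display until repaired by welding.
; A valid sender overlapping the weld trigger advances a repair timer that blends the cables' "Broken" morph target out, then enables the panel and starts the crane's camera capture.
; Child-actor push buttons drive the crane once enabled: held directional buttons shift its destination, and the grab button toggles grab/release.
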(event OnComponentBeginOverlap(WeldTrigger)
  (params (OverlappedComponent :type Primitive%20Component%20Object%20Reference) (OtherActor :type Actor%20Object%20Reference) (OtherComp :type Primitive%20Component%20Object%20Reference) (OtherBodyIndex :type Integer) (bFromSweep :type Boolean) (SweepResult :type Hit%20Result%20Structure%20%28by%20ref%29))
  (Default|CheckforValidSenderBeginOverlap (Variables|Default|GetBP_NFReceiverComponent) OtherActor))

(event OnComponentEndOverlap(WeldTrigger)
  (params (OverlappedComponent :type Primitive%20Component%20Object%20Reference) (OtherActor :type Actor%20Object%20Reference) (OtherComp :type Primitive%20Component%20Object%20Reference) (OtherBodyIndex :type Integer))
  (Default|CheckforValidSenderEndOverlap (Variables|Default|GetBP_NFReceiverComponent) OtherActor))

(event OnValidSenderTickOverlap(BP_NFReceiverComponent)
  (CallFunction|WeldTick))

(event Custom|WeldTick
  (if (< (Variables|Default|GetCurrentRepairTime) (Variables|Default|GetRepairTimeNeeded))
    (bind _output_get (Variables|Default|SetCurrentRepairTime (+ (Variables|Default|GetCurrentRepairTime) (Utilities|Time|GetWorldDeltaSeconds))))
    (Components|SkeletalMesh|SetMorphTarget (Variables|Default|GetSK_ControlPanelCables) "Broken" (- 1.0 (/ _output_get (Variables|Default|GetRepairTimeNeeded))) true)
    (else
      (CallFunction|EnablePanel))))

(event Custom|GrabButtonPress
  ;[1 0.9087 0 1 36] Bind grab button
  (if (Variables|Default|GetbIsEnabled)
    (Default|TryGrabbingorReleasing (Variables|Default|GetControlledCrane))))

(event EventBeginPlay
  (Utilities|FlowControl|Sequence
    (:then_0
      ;[1 0.9087 0 1 36] Bind grab button
      (bind _asbp_pushable_button (Utilities|Casting|CastToBP_PushableButton (Variables|/Script/Engine.ChildActorComponent|GetChildActor (Variables|Default|GetGrabButton))))
      (EventDispatchers|BindEventtoOnButtonPressed _asbp_pushable_button (delegate Custom|GrabButtonPress)))
    (:then_1
      (|BindMovementButtons))
    (:then_2
      ;[1 1 1] Set cables morph target to unrepaired
      (Components|SkeletalMesh|SetMorphTarget (Variables|Default|GetSK_ControlPanelCables) "Broken" 1.0 true)
      ;[1 1 1] Black out the display
      (Default|DrawMaterialtoRenderTarget (Variables|/Game/VRPuzzle/Gameplay/CargoBay/BeamCrane/BP_BeamCrane.BP_BeamCrane_C|GetBP_CameraCapturerComponent (Variables|Default|GetControlledCrane)) "/Game/VRPuzzle/Art/Environment/Station/CargoBay/CraneControlPanel/M_DisabledCamera.M_DisabledCamera"))))

(fn ConstructionScript)

(fn EnablePanel
  (if (not (Variables|Default|GetbIsEnabled))
    (Development|PrintString "Enabling crane control panel")
    ;[1 1 1] Start capturing on next tick
    (Default|StartCapturing (Variables|/Game/VRPuzzle/Gameplay/CargoBay/BeamCrane/BP_BeamCrane.BP_BeamCrane_C|GetBP_CameraCapturerComponent (Variables|Default|GetControlledCrane)))
    (Components|SkeletalMesh|SetMorphTarget (Variables|Default|GetSK_ControlPanelCables) "Broken" 0.0 true)
    (Variables|Default|SetbIsEnabled true)
    (return)))

(event Custom|TIckButtonBackwards
  ;[0.7166 0.7451 1 1 36] Bind Movement Buttons
  ;;[1 0.3521 0.9298] BInd Backwards Button
  (if (Variables|Default|GetbIsEnabled)
    (Default|ChangeCraneDestination (Variables|Default|GetControlledCrane) 0.0 (* (.y (Variables|Default|GetCraneDestinationChangeSpeed)) (Utilities|Time|GetWorldDeltaSeconds) -1.0))))

(event Custom|TickButtonRight
  ;[0.7166 0.7451 1 1 36] Bind Movement Buttons
  ;;[1 0.2904 0.2705] Bind Right Button
  (if (Variables|Default|GetbIsEnabled)
    (Default|ChangeCraneDestination (Variables|Default|GetControlledCrane) (* (.x (Variables|Default|GetCraneDestinationChangeSpeed)) (Utilities|Time|GetWorldDeltaSeconds) -1.0) 0.0)))

(event Custom|TickButtonLeft
  ;[0.7166 0.7451 1 1 36] Bind Movement Buttons
  ;;[0.1864 0.3194 1] Bind Left Button
  (if (Variables|Default|GetbIsEnabled)
    (Default|ChangeCraneDestination (Variables|Default|GetControlledCrane) (* (.x (Variables|Default|GetCraneDestinationChangeSpeed)) (Utilities|Time|GetWorldDeltaSeconds)) 0.0)))

(event Custom|TickButtonForwards
  ;[0.7166 0.7451 1 1 36] Bind Movement Buttons
  ;;[0.2711 1 0.2828] BInd Forwards Button
  (if (Variables|Default|GetbIsEnabled)
    (Default|ChangeCraneDestination (Variables|Default|GetControlledCrane) 0.0 (* (.y (Variables|Default|GetCraneDestinationChangeSpeed)) (Utilities|Time|GetWorldDeltaSeconds)))))