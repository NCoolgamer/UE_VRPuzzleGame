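; BP_BeamCrane is an overhead beam crane for the cargo bay that travels in a horizontal plane within a rectangular area.
; ChangeCraneDestination offsets the target, clamped to origin-centred bounds sized by two end markers.
; Each tick interpolates the head toward it at constant per-axis speeds, with the beams following only on Y.
; The construction script scales a bounds visualization to match the area.
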(event Custom|ChangeCraneDestination
  (params (DeltaX :type Float%20%28double-precision%29) (DeltaY :type Float%20%28double-precision%29))
  (CallFunction|ClampDestination (+ (Math|Vector|MakeVector DeltaX DeltaY 0.0) (Variables|Default|GetCraneDestination))))

(event EventBeginPlay
  (Variables|Default|SetCraneSpaceDimensions (Math|Conversions|ToVector2D(Vector) (Math|Vector|VectorGetAbs (- (Variables|/Script/Engine.SceneComponent|GetRelativeLocation (Variables|Default|GetCraneSpaceEndFar)) (Variables|/Script/Engine.SceneComponent|GetRelativeLocation (Variables|Default|GetCraneSpaceEndNear)))))))

(event EventTick
  (params (DeltaSeconds :type Float%20%28single-precision%29))
  (CallFunction|MoveCraneTick))

(fn ConstructionScript
  (Transformation|SetRelativeScale3D (Variables|Default|GetCraneMovementBoundsVisualization) (Math|Conversions|ToVector(Vector2D) (Math|Conversions|ToVector2D(Vector) (/ (Math|Vector|VectorGetAbs (- (Variables|/Script/Engine.SceneComponent|GetRelativeLocation (Variables|Default|GetCraneSpaceEndFar)) (Variables|/Script/Engine.SceneComponent|GetRelativeLocation (Variables|Default|GetCraneSpaceEndNear)))) (Math|Float|MakeLiteralFloat 1e+02))))))

(fn MoveCraneTick
  (bind _beams (Variables|Default|GetBeams))
  (bind _cranehead (Variables|Default|GetCraneHead))
  (bind _relativelocation (Variables|/Script/Engine.SceneComponent|GetRelativeLocation _beams))
  ;[1 1 1] Calculate the new Y location in local space
  (LocalVariables|SetNewY (Math|Interpolation|FInterptoConstant (.y (Variables|/Script/Engine.SceneComponent|GetRelativeLocation (Variables|Default|GetCraneHead))) (.y (Variables|Default|GetCraneDestination)) (Utilities|Time|GetWorldDeltaSeconds) (.y (Variables|Default|GetCraneMovementSpeed))))
  ;[1 1 1] Calculate the new X location in local space
  (LocalVariables|SetNewX (Math|Interpolation|FInterptoConstant (.x (Variables|/Script/Engine.SceneComponent|GetRelativeLocation (Variables|Default|GetCraneHead))) (.x (Variables|Default|GetCraneDestination)) (Utilities|Time|GetWorldDeltaSeconds) (.x (Variables|Default|GetCraneMovementSpeed))))
  (Utilities|FlowControl|Sequence
    (:then_0
      ;[1 1 1] Set beams location
      (Transformation|SetRelativeLocation _beams (Math|Vector|MakeVector (.x _relativelocation) (LocalVariables|GetNewY) (.z _relativelocation)) false false))
    (:then_1
      ;[1 1 1] Set Head location
      (Transformation|SetRelativeLocation _cranehead (Math|Vector|MakeVector (LocalVariables|GetNewX) (LocalVariables|GetNewY) (.z (Variables|/Script/Engine.SceneComponent|GetRelativeLocation _cranehead))) false false))))

(fn ClampDestination
  (params (NewDestination :type Vector))
  (bind _returnvalue (Math|Float|MakeLiteralFloat 2.0))
  (bind _cranespacedimensions (Variables|Default|GetCraneSpaceDimensions))
  (bind _returnvalue_2 (/ _cranespacedimensions _returnvalue))
  (bind _returnvalue_3 (Class|KismetMathLibrary|Negated2D _returnvalue_2))
  (bind (_x _y) (Math|Vector2D|BreakVector2D _returnvalue_2))
  (Variables|Default|SetCraneDestination (Math|Vector|MakeVector (Math|Float|Clamp(Float) (.x NewDestination) (.x _returnvalue_3) _x) (Math|Float|Clamp(Float) (.y NewDestination) (.y _returnvalue_3) _y) 0.0))
  (return))