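; Small sector gate actor in a VR puzzle game, with a widget screen that shows gate status and exit text and offers an exit button.
; On BeginPlay it passes its status and text to the WBP_SectorGate widget and binds to the exit button's click event.
; A click, or the debug simulate event, prints a message and fires the OnExitInitiated dispatcher.
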(event Custom|OnExitButtonClicked
  (Development|PrintString "Exit button clicked.")
  (Default|CallOnExitInitiated))

(event Custom|DEBUG%20SimulateExitButton
  (Development|PrintString "Exit button clicked.")
  (Default|CallOnExitInitiated))

(event EventBeginPlay
  (CallFunction|SetupScreen))

(event Collision|EventActorBeginOverlap
  (params (OtherActor :type Actor%20Object%20Reference)))

(event EventTick
  (params (DeltaSeconds :type Float%20%28single-precision%29)))

(fn ConstructionScript)

(fn SetupScreen
  (bind _aswbp_sector_gate (Utilities|Casting|CastToWBP_SectorGate (UserInterface|GetWidget (Variables|Default|GetGateScreen))))
  (Default|SetGateStatus _aswbp_sector_gate (Variables|Default|GetGateStatus))
  (Default|SetSectorExitTest _aswbp_sector_gate (Variables|Default|GetGateExitText))
  (EventDispatchers|BindEventtoOnExitButtonClicked _aswbp_sector_gate (EventDispatchers|CreateEvent :!event Custom|OnExitButtonClicked)))