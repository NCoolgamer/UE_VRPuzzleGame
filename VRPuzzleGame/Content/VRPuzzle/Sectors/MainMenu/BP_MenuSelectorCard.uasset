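; Main menu selector card in the VR puzzle game that shows only when its required sector is available in the save.
; On BeginPlay it caches the VR game instance, runs the visibility check and binds to the save data reload event.
; The check hides the actor in game unless the save's AvailableSectors contains its RequiredSectorId.
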(event Custom|CheckIfShouldBeVisible
  (Rendering|SetActorHiddenInGame (not (Utilities|Array|ContainsItem (Variables|/Game/VRPuzzle/Core/Saving/BP_StationGameSave.BP_StationGameSave_C|GetAvailableSectors (Variables|/Game/VRPuzzle/Core/Player/BP_VRGameInstance.BP_VRGameInstance_C|GetSaveGameInstance (Variables|Default|GetGameInstance))) (Variables|Default|GetRequiredSectorId)))))

(event EventBeginPlay
  (|CallParentFunction)
  (bind _asbp_vrgame_instance (Utilities|Casting|CastToBP_VRGameInstance (Game|GetGameInstance)))
  (Variables|Default|SetGameInstance _asbp_vrgame_instance)
  (CallFunction|CheckifShouldbeVisible)
  (EventDispatchers|BindEventtoOnSaveDataReload (Variables|Default|GetGameInstance) (EventDispatchers|CreateEvent :!event Custom|CheckIfShouldBeVisible)))

(event Collision|EventActorBeginOverlap
  (params (OtherActor :type Actor%20Object%20Reference))
  (|CallParentFunction OtherActor) ; This node is disabled and will not be called.\nDrag off pins to build functionality.
)

(event EventTick
  (params (DeltaSeconds :type Float%20%28single-precision%29))
  (|CallParentFunction DeltaSeconds) ; This node is disabled and will not be called.\nDrag off pins to build functionality.
)

(fn ConstructionScript
  (|CallParentFunction))