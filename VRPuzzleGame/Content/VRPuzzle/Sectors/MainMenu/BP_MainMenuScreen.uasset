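; Main menu screen actor for the VR puzzle game, showing a sector preview when a keycard is inserted.
; On begin play it caches its widget component's menu widget and emits a tap at the widget's location on button presses.
; An inserted keycard's ID looks up a row in the sector preview data table, which feeds the widget's preview screen.
; Removing keycards returns the widget to its main screen.
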(event Custom|ProcessKeycardsRemoved
  (if true
    (Default|ShowMainScreen (Variables|Default|GetMainMenuWidget))))

(event Custom|ProcessKeycardInserted
  (params (KeycardID :type String))
  (bind _returnvalue (Utilities|GetDataTableRow (Variables|Default|GetSectorPreviewInfos) (Utilities|String|StringToName KeycardID))
    (:then
      (Default|SwitchPreview (Variables|Default|GetMainMenuWidget) _returnvalue)
      (Default|ShowPreviewScreen (Variables|Default|GetMainMenuWidget)))))

(event Custom|EmitTap
  (CallFunction|EmitTapatLocation self (Transformation|GetWorldLocation (Variables|Default|GetWidget))))

(event EventBeginPlay
  (bind _aswbp_main_menu_screen (Utilities|Casting|CastToWBP_MainMenuScreen (UserInterface|GetWidget (Variables|Default|GetWidget))))
  (bind _output_get (Variables|Default|SetMainMenuWidget _aswbp_main_menu_screen))
  (EventDispatchers|BindEventtoOnButtonPressed _output_get (delegate Custom|EmitTap)))

(event Collision|EventActorBeginOverlap
  (params (OtherActor :type Actor%20Object%20Reference)))

(event EventTick
  (params (DeltaSeconds :type Float%20%28single-precision%29)))

(fn ConstructionScript)