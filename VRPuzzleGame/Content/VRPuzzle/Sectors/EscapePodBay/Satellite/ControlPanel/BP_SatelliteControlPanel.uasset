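; Control panel for the Escape Pod Bay satellite puzzle, where held buttons apply torque to a linked satellite to aim it at its target.
; A hologram mirrors the satellite's rotation, with Niagara beams showing target and current direction, the latter colored by alignment.
; Each tick, alignment sets signal strength on a linked status screen.
; Above a threshold it advances a curve-scaled transfer, otherwise progress resets; completion fires once.
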(event Custom|ButtonTickZU
  ;[0.9313 1 0.5782] Process button events
  (Default|AddTorqueVector (Variables|Default|GetLinkedSatellite) "0.000000,0.000000,1.000000"))

(event Custom|ButtonTickZD
  ;[0.9313 1 0.5782] Process button events
  (Default|AddTorqueVector (Variables|Default|GetLinkedSatellite) "0.000000,0.000000,-1.000000"))

(event Custom|ButtonTickR
  ;[0.9313 1 0.5782] Process button events
  (Default|AddTorqueVector (Variables|Default|GetLinkedSatellite) "0.000000,-1.000000,0.000000"))

(event Custom|ButtonTickL
  ;[0.9313 1 0.5782] Process button events
  (Default|AddTorqueVector (Variables|Default|GetLinkedSatellite) "0.000000,1.000000,0.000000"))

(event Custom|ButtonTickU
  ;[0.9313 1 0.5782] Process button events
  (Default|AddTorqueVector (Variables|Default|GetLinkedSatellite) "-1.000000,0.000000,0.000000"))

(event Custom|ButtonTickD
  ;[0.9313 1 0.5782] Process button events
  (Default|AddTorqueVector (Variables|Default|GetLinkedSatellite) "1.000000,0.000000,0.000000"))

(event EventBeginPlay
  (Utilities|FlowControl|DelayUntilNextTick)
  (CallFunction|UpdateTargetBeam)
  (Components|Activation|Activate (Variables|Default|GetNS_SatelliteCurrent) false)
  (Components|Activation|Activate (Variables|Default|GetNS_SatelliteTarget) false))

(event Collision|EventActorBeginOverlap
  (params (OtherActor :type Actor%20Object%20Reference)))

(event EventTick
  (params (DeltaSeconds :type Float%20%28single-precision%29))
  (bind _linkedsatellite (Variables|Default|GetLinkedSatellite))
  (bind _lastdotproduct (Variables|/Game/VRPuzzle/Sectors/EscapePodBay/Satellite/BP_Satellite.BP_Satellite_C|GetLastDotProduct _linkedsatellite))
  (bind _returnvalue (Math|Float|Max(Float) _lastdotproduct 0.0))
  ;[1 1 1] Align hologram to actual satellite
  (Transformation|SetWorldRotation (Variables|Default|GetS_Satellite) (Transformation|GetWorldRotation (Variables|/Game/VRPuzzle/Sectors/EscapePodBay/Satellite/BP_Satellite.BP_Satellite_C|GetMainPart (Variables|Default|GetLinkedSatellite))) false false)
  (CallFunction|UpdateCurrentBeam)
  (Default|SetAngularVelocityText (Variables|/Game/VRPuzzle/Sectors/EscapePodBay/Satellite/ControlPanel/BP_SatelliteStatusScreen.BP_SatelliteStatusScreen_C|GetStatusScreenWidget (Variables|Default|GetStatus%20Screen)) (Default|GetCurrentVelocity (Variables|Default|GetLinkedSatellite)))
  (Default|SetSignalStrengthText (Variables|/Game/VRPuzzle/Sectors/EscapePodBay/Satellite/ControlPanel/BP_SatelliteStatusScreen.BP_SatelliteStatusScreen_C|GetStatusScreenWidget (Variables|Default|GetStatus%20Screen)) _returnvalue)
  (CallFunction|UpdateTransferProgress _returnvalue)
  (if (>= (Variables|Default|GetCurrentTransferProgress) 1.0)
    ;[0.07438 1 0] Tranfer completed
    (Utilities|FlowControl|DoOnce false
      (:Completed
        (Default|CallOnTransferComplete)
        (CallFunction|EmitSuccessorErroratLocation true self (Transformation|GetWorldLocation (Variables|/Game/VRPuzzle/Sectors/EscapePodBay/Satellite/ControlPanel/BP_SatelliteStatusScreen.BP_SatelliteStatusScreen_C|GetStatusWidget (Variables|Default|GetStatus%20Screen))))
        (Development|PrintText "Transfer Successful!")))))

(fn ConstructionScript)

(fn LinktoSatellite
  (params (Satellite :type BP%20Satellite%20Object%20Reference))
  (Variables|Default|SetLinkedSatellite Satellite)
  (Utilities|FlowControl|Sequence
    (:then_0
      ;[1 1 1 1 36] Bind rotator buttons
      ;;[1 0.04598 0] X Buttons
      (bind _asbp_pushable_button (Utilities|Casting|CastToBP_PushableButton (Variables|/Script/Engine.ChildActorComponent|GetChildActor (Variables|Default|GetButtonL))))
      (EventDispatchers|BindEventtoOnButtonHeldTick _asbp_pushable_button (EventDispatchers|CreateEvent :!event Custom|ButtonTickL)))
    (:then_1
      (bind _asbp_pushable_button_2 (Utilities|Casting|CastToBP_PushableButton (Variables|/Script/Engine.ChildActorComponent|GetChildActor (Variables|Default|GetButtonR))))
      (EventDispatchers|BindEventtoOnButtonHeldTick _asbp_pushable_button_2 (EventDispatchers|CreateEvent :!event Custom|ButtonTickR)))
    (:then_2
      ;;[0.09334 1 0] Y Buttons
      (bind _asbp_pushable_button_3 (Utilities|Casting|CastToBP_PushableButton (Variables|/Script/Engine.ChildActorComponent|GetChildActor (Variables|Default|GetButtonD))))
      (EventDispatchers|BindEventtoOnButtonHeldTick _asbp_pushable_button_3 (EventDispatchers|CreateEvent :!event Custom|ButtonTickD)))
    (:then_3
      (bind _asbp_pushable_button_4 (Utilities|Casting|CastToBP_PushableButton (Variables|/Script/Engine.ChildActorComponent|GetChildActor (Variables|Default|GetButtonU))))
      (EventDispatchers|BindEventtoOnButtonHeldTick _asbp_pushable_button_4 (EventDispatchers|CreateEvent :!event Custom|ButtonTickU)))
    (:then_4
      ;;[0.1522 0.1102 1] Z buttons
      (bind _asbp_pushable_button_5 (Utilities|Casting|CastToBP_PushableButton (Variables|/Script/Engine.ChildActorComponent|GetChildActor (Variables|Default|GetButtonZD))))
      (EventDispatchers|BindEventtoOnButtonHeldTick _asbp_pushable_button_5 (EventDispatchers|CreateEvent :!event Custom|ButtonTickZD)))
    (:then_5
      (bind _asbp_pushable_button_6 (Utilities|Casting|CastToBP_PushableButton (Variables|/Script/Engine.ChildActorComponent|GetChildActor (Variables|Default|GetButtonZU))))
      (EventDispatchers|BindEventtoOnButtonHeldTick _asbp_pushable_button_6 (EventDispatchers|CreateEvent :!event Custom|ButtonTickZU))
      (return))))

(fn UpdateTargetBeam
  (Niagara|SetNiagaraVariable(Vector3) (Variables|Default|GetNS_SatelliteTarget) "BeamEnd" (+ (Transformation|GetWorldLocation (Variables|Default|GetNS_SatelliteTarget)) (* (Default|GetUnitVectorfromSatellitetoTarget (Variables|Default|GetLinkedSatellite)) (Variables|Default|GetHologramBeamLength)))))

(fn UpdateCurrentBeam
  (Niagara|SetNiagaraVariable(Vector3) (Variables|Default|GetNS_SatelliteCurrent) "BeamEnd" (+ (Transformation|GetWorldLocation (Variables|Default|GetNS_SatelliteCurrent)) (* (Default|GetCurrentPointDirection (Variables|Default|GetLinkedSatellite)) (Variables|Default|GetHologramBeamLength))))
  (Niagara|SetNiagaraVariable(LinearColor) (Variables|Default|GetNS_SatelliteCurrent) "BeamColor" (Math|Curves|GetLinearColorValue (Variables|Default|GetHologramCurrentBeamColorCurve) (Variables|/Game/VRPuzzle/Sectors/EscapePodBay/Satellite/BP_Satellite.BP_Satellite_C|GetLastDotProduct (Variables|Default|GetLinkedSatellite)))))

(fn LinktoStatusScreen
  (params (StatusScreen :type BP%20Satellite%20Status%20Screen%20Object%20Reference))
  (Variables|Default|SetStatus%20Screen StatusScreen))

(fn UpdateTransferProgress
  (params (CurrentSignalStrength :type Float%20%28double-precision%29))
  (Utilities|FlowControl|Sequence
    (:then_0
      (if (>= CurrentSignalStrength (Variables|Default|GetUplinkActivationStrengthThreshold))
        (Variables|Default|SetCurrentTransferProgress (Math|Float|Min(Float) (+ (Variables|Default|GetCurrentTransferProgress) (/ (* (Utilities|Time|GetWorldDeltaSeconds) (Math|Curves|GetFloatValue (Variables|Default|GetTransferSpeedMultiplierCurve) CurrentSignalStrength)) (Variables|Default|GetTransferTime))) 1.0))
        (else
          ;[1 1 1] Reset progress
          (Variables|Default|SetCurrentTransferProgress 0.0))))
    (:then_1
      ;[1 1 1] Update UI
      (Default|SetTransferProgressValue (Variables|/Game/VRPuzzle/Sectors/EscapePodBay/Satellite/ControlPanel/BP_SatelliteStatusScreen.BP_SatelliteStatusScreen_C|GetStatusScreenWidget (Variables|Default|GetStatus%20Screen)) (Variables|Default|GetCurrentTransferProgress)))))