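; Physics-rotated satellite in the Escape Pod Bay VR puzzle that the player aims at a target, with assisted alignment.
; Torque events apply angular impulses to the main part, and BeginPlay computes the target rotation from the target's location.
; Each tick, the dot product between the part's up vector and target direction drives a curve-based RInterpTo snap assist, active only at low linear velocity.
; Debug arrows and push events support testing.
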(event Custom|PushCCW_Z
  ;[0.4058 1 0] DEBUG
  (Alignment|AddAngularImpulse "0.000000,0.000000,-1.000000" (Variables|Default|GetRotationForce)))

(event Custom|PushCW_Z
  ;[0.4058 1 0] DEBUG
  (Alignment|AddAngularImpulse "0.000000,0.000000,1.000000" (Variables|Default|GetRotationForce)))

(event Custom|AddTorqueVector
  (params (TorqueDirection :type Vector))
  (Alignment|AddAngularImpulse TorqueDirection (* (Variables|Default|GetRotationForce) (Utilities|Time|GetWorldDeltaSeconds))))

(event Custom|DEBUG%20Set%20RotationToTarget
  ;[0.4058 1 0] DEBUG
  (Transformation|SetWorldRotation (Variables|Default|GetMainPart) (Variables|Default|GetTargetRotation) false false))

(event Custom|PushCW_X
  ;[0.4058 1 0] DEBUG
  (Alignment|AddAngularImpulse "1.000000,0.000000,0.000000" (Variables|Default|GetRotationForce)))

(event Custom|PushCCW_X
  ;[0.4058 1 0] DEBUG
  (Alignment|AddAngularImpulse "-1.000000,0.000000,0.000000" (Variables|Default|GetRotationForce)))

(event Custom|PushCW_Y
  ;[0.4058 1 0] DEBUG
  (Alignment|AddAngularImpulse "0.000000,1.000000,0.000000" (Variables|Default|GetRotationForce)))

(event Custom|PushCCW_Y
  ;[0.4058 1 0] DEBUG
  (Alignment|AddAngularImpulse "0.000000,-1.000000,0.000000" (Variables|Default|GetRotationForce)))

(event EventBeginPlay
  (Alignment|RecalculateTargetRotation))

(event EventTick
  (params (DeltaSeconds :type Float%20%28single-precision%29))
  (Debug|DrawDebugArrows)
  ;[1 1 1] Recalculate the alignment
  (Variables|Default|SetLastDotProduct (Alignment|CalculateDottoTarget))
  ;[1 1 1] Show debug values
  (Development|PrintText (Utilities|Text|ToText(Float) (Variables|Default|GetLastDotProduct) "HalfToEven") true true "(R=0.000000,G=0.660000,B=1.000000,A=1.000000)" 2.0 "ANGLE")
  (Development|PrintText (Utilities|Text|ToText(Float) (Class|KismetMathLibrary|VectorHeadingAngle (Alignment|GetCurrentPointDirection)) "HalfToEven") true true "(R=0.673462,G=1.000000,B=0.000000,A=1.000000)" 2.0 "HDG")
  ;[0.6353 0.6225 1] Align to target if close enough
  (if (and (not (<= (Math|Curves|GetFloatValue (Variables|Default|GetRotationHelpStrengthCurve) (Variables|Default|GetLastDotProduct)) 1e-06)) (<= (Math|Vector|VectorLength (Alignment|GetCurrentVelocity)) (Variables|Default|GetMaxVelocityForHelp)))
    (Transformation|SetWorldRotation (Variables|Default|GetMainPart) (Math|Interpolation|RInterpTo (Transformation|GetWorldRotation (Variables|Default|GetMainPart)) (Variables|Default|GetTargetRotation) (Utilities|Time|GetWorldDeltaSeconds) (Math|Curves|GetFloatValue (Variables|Default|GetRotationHelpStrengthCurve) (Variables|Default|GetLastDotProduct))) false false)))

(fn ConstructionScript)

(fn AddAngularImpulse
  (params (ImpulseDirection :type Vector) (Multiplier :type Float%20%28double-precision%29))
  (Class|PrimitiveComponent|AddAngularImpulseinDegrees (Variables|Default|GetMainPart) (* ImpulseDirection Multiplier) "None" true))

(fn DrawDebugVector
  (params (Origin :type Vector) (ForwardVector :type Vector))
  (Rendering|Debug|DrawDebugArrow Origin (+ Origin (* ForwardVector (Math|Float|MakeLiteralFloat 1e+05))) 1e+03 "(R=1.000000,G=0.000000,B=0.603579,A=1.000000)" 0.0 2e+01))

(fn GetUnitVectorfromSatellitetoTarget
  (return (Math|Vector|ClampVectorSize (- (Transformation|GetWorldLocation (Variables|Default|GetSatelliteTarget)) (Transformation|GetWorldLocation (Variables|Default|GetMainPart))) 0.0 1.0)))

(fn GetCurrentPointDirection
  (return (Math|Vector|GetUpVector (Variables|Default|GetMainPart))))

(fn CalculateDottoTarget
  (return (Math|Vector|DotProduct (Alignment|GetUnitVectorfromSatellitetoTarget) (Alignment|GetCurrentPointDirection))))

(fn DrawDebugArrows
  (Debug|DrawDebugVector (Transformation|GetWorldLocation (Variables|Default|GetMainPart)) (Alignment|GetCurrentPointDirection))
  (Debug|DrawDebugVector (Transformation|GetWorldLocation (Variables|Default|GetSatelliteTarget)) (Math|Vector|NegateVector (Alignment|GetUnitVectorfromSatellitetoTarget))))

(fn RecalculateTargetRotation
  (Variables|Default|SetTargetRotation (Math|Rotator|CombineRotators "0.000000,-90.000000,-90.000000" (Math|Rotator|FindLookatRotation (Transformation|GetWorldLocation (Variables|Default|GetSatelliteTarget)) (Transformation|GetWorldLocation (Variables|Default|GetMainPart))))))

(fn GetCurrentVelocity
  (return (Transformation|GetComponentVelocity (Variables|Default|GetMainPart))))