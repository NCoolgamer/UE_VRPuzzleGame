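; BP_PodPower is the escape pod's power cell receptacle in a VR puzzle, behind a grate that is grabbed and moved along a spline.
; The receiver component accepts senders only while the grate is open past a minimum amount.
; Box overlaps feed the receiver, which powers the pod on for a charged cell ID and off when a valid sender leaves.
; Power state is broadcast on BeginPlay and on those sender events.
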(event OnComponentBeginOverlap(Box)
  (params (OverlappedComponent :type Primitive%20Component%20Object%20Reference) (OtherActor :type Actor%20Object%20Reference) (OtherComp :type Primitive%20Component%20Object%20Reference) (OtherBodyIndex :type Integer) (bFromSweep :type Boolean) (SweepResult :type Hit%20Result%20Structure%20%28by%20ref%29))
  (Default|CheckforValidSenderBeginOverlap (Variables|Default|GetBP_NFReceiverComponent) OtherActor))

(event OnComponentEndOverlap(Box)
  (params (OverlappedComponent :type Primitive%20Component%20Object%20Reference) (OtherActor :type Actor%20Object%20Reference) (OtherComp :type Primitive%20Component%20Object%20Reference) (OtherBodyIndex :type Integer))
  (Default|CheckforValidSenderEndOverlap (Variables|Default|GetBP_NFReceiverComponent) OtherActor))

(event OnValidSenderBeginOverlap(BP_NFReceiverComponent)
  (bind _lastacceptedid (Default|GetLastValidSenderID (Variables|Default|GetBP_NFReceiverComponent)))
  (Variables|Default|SetbPoweredOn (Utilities|Enum|Equal(Enum) _lastacceptedid (Variables|Default|GetPowerCellChargedID)))
  (Default|CallOnPowerStateChanged (Variables|Default|GetbPoweredOn)))

(event OnSplineLockedMoved(GrabComponent)
  (params (TImeAlongSpline :type Float%20%28double-precision%29))
  (Variables|/Game/VRPuzzle/Core/Interactables/NearFieldInteraction/BP_NFReceiverComponent.BP_NFReceiverComponent_C|SetbCanAcceptSenders (Variables|Default|GetBP_NFReceiverComponent) (>= TImeAlongSpline (Variables|Default|GetMinimumOpeningForHolding))))

(event OnValidSenderEndOverlap(BP_NFReceiverComponent)
  (params (ValidSendersLeft :type Integer))
  (Variables|Default|SetbPoweredOn false)
  (Default|CallOnPowerStateChanged (Variables|Default|GetbPoweredOn)))

(event EventBeginPlay
  (Variables|/Game/VRPuzzle/Core/Grabbing/GrabComponent.GrabComponent_C|SetTargetSpline (Variables|Default|GetGrabComponent) (Variables|Default|GetGrateMovementSpline))
  (Default|CallOnPowerStateChanged (Variables|Default|GetbPoweredOn)))

(event Collision|EventActorBeginOverlap
  (params (OtherActor :type Actor%20Object%20Reference)))

(event EventTick
  (params (DeltaSeconds :type Float%20%28single-precision%29)))

(fn ConstructionScript)

(fn GetHoldPointComponent
  (return (Variables|Default|GetPowerCellHoldPoint)))