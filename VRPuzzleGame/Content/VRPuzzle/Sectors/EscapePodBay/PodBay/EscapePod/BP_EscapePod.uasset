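; Escape pod actor for the VR puzzle's pod bay, with a lockable animated door and a launch that carries the player along.
; It binds to door and control monitor widgets for open and launch events, starting with the door locked.
; Paired DoOnce nodes alternate opening and closing, toggling animation and collision.
; Launching enables Tick, which offsets both pod and player pawn along the launch axis; debug events test unlocking and launch.
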(event Custom|OpenDoor
  ;[1 1 1 1 36] Door operation
  (Utilities|FlowControl|DoOnce false
    (:Completed
      (CallFunction|EmitSuccessorErroratLocation true self (Transformation|GetWorldLocation (Variables|Default|GetDoorWidget)))
      (Components|Animation|PlayAnimation (Variables|Default|GetPodDoor) "/Game/VRPuzzle/Sectors/EscapePodBay/PodBay/EscapePod/Animations/AS_OpenPodDoor.AS_OpenPodDoor" false)
      (Collision|SetCollisionEnabled (Variables|Default|GetInsideCollision) "NoCollision")
      (Collision|SetCollisionEnabled (Variables|Default|GetDoorCollision) "NoCollision")
      (Utilities|FlowControl|DoOnce true) ; enters at Reset
    )))

(event Custom|CloseDoor
  ;[1 1 1 1 36] Door operation
  (Utilities|FlowControl|DoOnce true
    (:Completed
      (Components|Animation|PlayAnimation (Variables|Default|GetPodDoor) "/Game/VRPuzzle/Sectors/EscapePodBay/PodBay/EscapePod/Animations/AS_ClosePodDoor.AS_ClosePodDoor" false)
      (Collision|SetCollisionEnabled (Variables|Default|GetInsideCollision) "QueryAndPhysics")
      (Collision|SetCollisionEnabled (Variables|Default|GetDoorCollision) "QueryAndPhysics")
      (Utilities|FlowControl|DoOnce false) ; enters at Reset
    )))

(event Custom|SetDoorLockedState
  (params (bLockdownActive :type Boolean))
  ;[1 1 1 1 36] Door operation
  (Default|SwitchLockedState (Variables|Default|GetEscapePodDoorWidget) bLockdownActive))

(event Custom|DEBUG%20UnlockDoor
  ;[0 1 0.003062] DEBUG
  (Default|SwitchLockedState (Variables|Default|GetEscapePodDoorWidget) false))

(event Custom|LaunchPod
  ;[0.4453 0.4849 1] Launch
  (Actor|Tick|SetActorTickEnabled true))

(event Custom|DEBUG%20StartLaunchSequence
  ;[0 1 0.003062] DEBUG
  (Default|StartLaunchSequence (Variables|Default|GetPodControlMonitorWidget)))

(event EventBeginPlay
  ;[1 1 1] Link up with the door widget
  (bind _aswbp_escape_pod_door (Utilities|Casting|CastToWBP_EscapePodDoor (UserInterface|GetWidget (Variables|Default|GetDoorWidget))))
  (bind _output_get (Variables|Default|SetEscapePodDoorWidget _aswbp_escape_pod_door))
  (Default|SwitchLockedState _output_get true)
  (EventDispatchers|BindEventtoOnOpenButtonPressed (Variables|Default|GetEscapePodDoorWidget) (EventDispatchers|CreateEvent :!event Custom|OpenDoor))
  (bind _aswbp_escape_pod_control_monitor (Utilities|Casting|CastToWBP_EscapePodControlMonitor (UserInterface|GetWidget (Variables|Default|GetControlScreenWidget))))
  (bind _output_get_2 (Variables|Default|SetPodControlMonitorWidget _aswbp_escape_pod_control_monitor))
  (EventDispatchers|BindEventtoOnLaunch _output_get_2 (EventDispatchers|CreateEvent :!event Custom|LaunchPod)))

(event EventTick
  (params (DeltaSeconds :type Float%20%28single-precision%29))
  (bind _launchspeed (Variables|Default|GetLaunchSpeed))
  (bind _launchaxis (Variables|Default|GetLaunchAxis))
  (bind _returnvalue (* DeltaSeconds _launchspeed))
  (bind _returnvalue_2 (* _returnvalue _launchaxis))
  ;[0.4453 0.4849 1] Launch
  (Transformation|AddWorldOffset (Variables|Default|GetDefaultSceneRoot) _returnvalue_2 false false)
  (Transformation|AddWorldOffset (Variables|/Script/Engine.Actor|GetRootComponent (Game|Player|GetPlayerPawn 0)) _returnvalue_2 false false))

(fn ConstructionScript)