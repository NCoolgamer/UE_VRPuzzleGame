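; BP_PowerCellCharger is a VR puzzle station that charges power cells when its button is pressed with the port door closed.
; A grab component rotates the door, whose angle or overlap with a closed-position collider sets the port state shown on a widget.
; A box overlap feeds a receiver component that tracks cells in range.
; Charging sets those cells charged and plays a sound, with DoOnce and a delay as cooldown.
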(event OnComponentBeginOverlap(Box)
  (params (OverlappedComponent :type Primitive%20Component%20Object%20Reference) (OtherActor :type Actor%20Object%20Reference) (OtherComp :type Primitive%20Component%20Object%20Reference) (OtherBodyIndex :type Integer) (bFromSweep :type Boolean) (SweepResult :type Hit%20Result%20Structure%20%28by%20ref%29))
  (Default|CheckforValidSenderBeginOverlap (Variables|Default|GetBP_NFReceiverComponent) OtherActor))

(event OnComponentEndOverlap(Box)
  (params (OverlappedComponent :type Primitive%20Component%20Object%20Reference) (OtherActor :type Actor%20Object%20Reference) (OtherComp :type Primitive%20Component%20Object%20Reference) (OtherBodyIndex :type Integer))
  (Default|CheckforValidSenderEndOverlap (Variables|Default|GetBP_NFReceiverComponent) OtherActor))

(event OnComponentBeginOverlap(PortClosedCollision)
  (params (OverlappedComponent :type Primitive%20Component%20Object%20Reference) (OtherActor :type Actor%20Object%20Reference) (OtherComp :type Primitive%20Component%20Object%20Reference) (OtherBodyIndex :type Integer) (bFromSweep :type Boolean) (SweepResult :type Hit%20Result%20Structure%20%28by%20ref%29))
  ;[1 1 1] Set port to closed when door is colliding with the closed collision
  (if (== OtherComp (Variables|Default|GetS_PowerCellChargerDoor))
    (bind _output_get (Variables|Default|SetbPortOpen false))
    (Default|SetPortOpenState (Variables|Default|GetChargerWidget) _output_get)))

(event Custom|ChargeCells
  (bind _bp_nfreceivercomponent (Variables|Default|GetBP_NFReceiverComponent))
  (bind _currentsenders (Variables|/Game/VRPuzzle/Core/Interactables/NearFieldInteraction/BP_NFReceiverComponent.BP_NFReceiverComponent_C|GetCurrentSenders _bp_nfreceivercomponent))
  ;[1 0.7682 0.3833] Charge all cells in range
  (Utilities|FlowControl|DoOnce false :!label _label
    (:Completed
      (if (not (Variables|Default|GetbPortOpen))
        (for _array_element _currentsenders
          (bind _asbp_power_cell (Utilities|Casting|CastToBP_PowerCell _array_element))
          (Default|SetChargedState _asbp_power_cell true))
        (if (> (Utilities|Array|Length _currentsenders) 0)
          (Audio|PlaySoundatLocation "/Game/VRPuzzle/Sectors/EscapePodBay/PodBay/PowerCell/Audio/S_PowerCharge_Cue.S_PowerCharge_Cue" (Transformation|GetWorldLocation (Variables|Default|GetPortClosedCollision)) "0, 0, 0" 1.0 1.0 0.0 0 0 0 0))
        (Utilities|FlowControl|Delay (Variables|Default|GetMinTimeBetweenCharges)) ; Allow charging once per X seconds
        (goto _label Reset)))))

(event Custom|OnPortRotated
  (params (NewRelativeAngle :type Float%20%28double-precision%29))
  ;[1 1 1] Set door closed based on angle
  (Development|PrintString (Utilities|String|ToString(Float) NewRelativeAngle))
  (bind _output_get (Variables|Default|SetbPortOpen (>= NewRelativeAngle (Variables|Default|GetPortOpenAngle))))
  (Development|PrintString (Utilities|String|SelectString "OPEN" "CLOSED" _output_get) true true (Math|Color|SelectColor "(R=0.176475,G=1.000000,B=0.000000,A=1.000000)" "(R=1.000000,G=0.027276,B=0.000000,A=1.000000)" _output_get) 2.0 "PORT")
  (Default|SetPortOpenState (Variables|Default|GetChargerWidget) (Variables|Default|GetbPortOpen)))

(event EventBeginPlay
  (Variables|/Game/VRPuzzle/Core/Grabbing/BP_GrabComponent.BP_GrabComponent_C|SetComponentToRotate (Variables|Default|GetGrabComponent) (Variables|Default|GetS_PowerCellChargerDoor))
  (EventDispatchers|BindEventtoOnRotated (Variables|Default|GetGrabComponent) (EventDispatchers|CreateEvent :!event Custom|OnPortRotated))
  ;[1 1 1] Bind to charge button
  (bind _asbp_pushable_button (Utilities|Casting|CastToBP_PushableButton (Variables|/Script/Engine.ChildActorComponent|GetChildActor (Variables|Default|GetBP_PushableButton))))
  (EventDispatchers|BindEventtoOnButtonPressed _asbp_pushable_button (EventDispatchers|CreateEvent :!event Custom|ChargeCells))
  (bind _aswbp_power_cell_charger (Utilities|Casting|CastToWBP_PowerCellCharger (UserInterface|GetWidget (Variables|Default|GetWidget))))
  (Variables|Default|SetChargerWidget _aswbp_power_cell_charger)
  (Default|SetPortOpenState (Variables|Default|GetChargerWidget) (Variables|Default|GetbPortOpen)))

(event Collision|EventActorBeginOverlap
  (params (OtherActor :type Actor%20Object%20Reference)))

(event EventTick
  (params (DeltaSeconds :type Float%20%28single-precision%29)))

(fn ConstructionScript)