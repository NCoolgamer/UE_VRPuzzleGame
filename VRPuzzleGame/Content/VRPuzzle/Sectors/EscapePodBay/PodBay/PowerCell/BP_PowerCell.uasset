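; BP_PowerCell is a grabbable VR puzzle power cell that is either charged or depleted, shown through a dynamic material parameter.
; Its holdable component lets receivers in range hold it, pausing while the player grabs it and auto-holding again on drop.
; The charge state selects the sender ID the cell returns.
; On auto-respawn, it copies charge state and both sender IDs to the replacement actor.
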(event OnGrabbed(GrabComponent)
  ;[1 1 1] Make sure the cell can't be held by other objects if held by the player
  (Variables|/Game/VRPuzzle/Core/Interactables/ItemHolder/BP_HoldableItemComponent.BP_HoldableItemComponent_C|SetbCanBeHeld (Variables|Default|GetBP_HoldableItemComponent) false))

(event OnDropped(GrabComponent)
  ;[1 1 1] Re-enable holding and auto-hold when possible
  (Variables|/Game/VRPuzzle/Core/Interactables/ItemHolder/BP_HoldableItemComponent.BP_HoldableItemComponent_C|SetbCanBeHeld (Variables|Default|GetBP_HoldableItemComponent) true)
  (Variables|/Game/VRPuzzle/Core/Interactables/ItemHolder/BP_HoldableItemComponent.BP_HoldableItemComponent_C|SetbTryToHoldUntilHeld (Variables|Default|GetBP_HoldableItemComponent) true))

(event OnRespawnedActorCreated(BP_AutoRespawnComponent)
  (params (RespawnedActor :type Actor%20Object%20Reference))
  (bind _asbp_power_cell (Utilities|Casting|CastToBP_PowerCell RespawnedActor))
  (Utilities|FlowControl|Sequence
    (:then_0
      (CallFunction|SetChargedState _asbp_power_cell (Variables|Default|GetbIsCharged)))
    (:then_1
      (Variables|BP_PowerCell_C|SetSenderIdCharged _asbp_power_cell (Variables|Default|GetSenderIdCharged)))
    (:then_2
      (Variables|BP_PowerCell_C|SetSenderIdDepleted _asbp_power_cell (Variables|Default|GetSenderIdDepleted)))))

(event OnTryGrab(GrabComponent)
  (Default|EndHold (Variables|Default|GetBP_HoldableItemComponent)))

(event EventBeginPlay
  (Variables|/Game/VRPuzzle/Core/Interactables/ItemHolder/BP_HoldableItemComponent.BP_HoldableItemComponent_C|SetItemPhysicsComponent (Variables|Default|GetBP_HoldableItemComponent) (Variables|Default|GetS_PowerCell))
  (Variables|/Game/VRPuzzle/Core/Interactables/ItemHolder/BP_HoldableItemComponent.BP_HoldableItemComponent_C|SetbTryToHoldUntilHeld (Variables|Default|GetBP_HoldableItemComponent) true)
  (bind _returnvalue (Rendering|Material|CreateDynamicMaterialInstance (Variables|Default|GetS_PowerCell) 1 0 "None" :!class /Script/Engine.PrimitiveComponent))
  (bind _output_get (Variables|Default|SetCellMaterial _returnvalue))
  (Rendering|Material|SetMaterial (Variables|Default|GetS_PowerCell) 1 _output_get)
  (CallFunction|UpdateMaterial))

(event Collision|EventActorBeginOverlap
  (params (OtherActor :type Actor%20Object%20Reference)))

(event EventTick
  (params (DeltaSeconds :type Float%20%28single-precision%29)))

(event EventReportReceiver
  (params (ReceiverComponent :type BP%20NF%20Receiver%20Component%20Object%20Reference) (bInRange :type Boolean))
  (Default|ProcessReceiverReport (Variables|Default|GetBP_HoldableItemComponent) ReceiverComponent bInRange))

(fn ConstructionScript)

(fn UpdateMaterial
  (Rendering|Material|SetScalarParameterValue (Variables|Default|GetCellMaterial) "ChargePercent" (Math|Float|SelectFloat 1.0 0.0 (Variables|Default|GetbIsCharged)) :!class /Script/Engine.MaterialInstanceDynamic))

(fn SetChargedState
  (params (bIsCharged :type Boolean))
  (Variables|Default|SetbIsCharged bIsCharged)
  (CallFunction|UpdateMaterial))

(fn GetSenderID
  (return (Utilities|String|SelectString (Variables|Default|GetSenderIdCharged) (Variables|Default|GetSenderIdDepleted) (Variables|Default|GetbIsCharged))))

(fn ShouldCallTick
  (return false))