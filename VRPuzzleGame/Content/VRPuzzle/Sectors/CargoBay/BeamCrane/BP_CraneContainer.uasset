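; BP_CraneContainer is a cargo crate actor in the Cargo Bay beam crane sector, exposing what is needed for it to be grabbed.
; Getter functions return its CanBeGrabbed flag, the GrabPoint component, and its Extents with the world-space offset from SCargoCrate to GrabPoint.
; A SetCollisionStatus event toggles collision for the whole actor.
; It holds no movement or grab logic of its own.
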(event EventBeginPlay
  (|CallParentFunction) ; This node is disabled and will not be called.\nDrag off pins to build functionality.
)

(event Collision|EventActorBeginOverlap
  (params (OtherActor :type Actor%20Object%20Reference)))

(event EventTick
  (params (DeltaSeconds :type Float%20%28single-precision%29))
  (|CallParentFunction DeltaSeconds) ; This node is disabled and will not be called.\nDrag off pins to build functionality.
)

(event EventSetCollisionStatus
  (params (bShouldCollide :type Boolean))
  (Collision|SetActorEnableCollision bShouldCollide))

(fn ConstructionScript
  (|CallParentFunction))

(fn GetCanbeGrabbed
  (return (Variables|Default|GetbCanBeGrabbed)))

(fn TryGetExtents
  (return (Variables|Default|GetExtents) (- (Transformation|GetWorldLocation (Variables|Default|GetGrabPoint)) (Transformation|GetWorldLocation (Variables|Default|GetS_CargoCrate)))))

(fn TryGetGrabPointComponent
  (return (Variables|Default|GetGrabPoint)))