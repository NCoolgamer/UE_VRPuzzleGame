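; Controllable overhead beam crane for the VR puzzle cargo bay that picks up and places grabbable actors within a bounded space.
; Tick interpolates beams, head and picker toward a clamped destination, with servo volume following movement speed.
; Box traces find targets and validate lifting, placing and carried-object movement.
; Destination-reached callbacks sequence attach, detach and retraction while controls lock, and a scene capture feeds a crane camera render target.
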(event Custom|PlaceLocationReached
  (bind _targetgrabbableactor (Variables|Grabbing|Current|GetTargetGrabbableActor))
  (bind _cranedestination (Variables|Movement|GetCraneDestination))
  ;[1 1 1] Placing object Callback
  (EventDispatchers|UnbindEventfromOnDestinationReached (delegate Custom|PlaceLocationReached))
  ;;[1 1 1] Detach and re-enable collision
  (Utilities|IsValid _targetgrabbableactor
    (:Is%20Valid
      (Transformation|DetachFromActor _targetgrabbableactor "KeepWorld" "KeepWorld" "KeepWorld")
      (Class|BPICraneGrabbable|SetCollisionStatus(Message) (Variables|Grabbing|Current|GetTargetGrabbableActor) true)
      ;;[1 1 1] Forget that we are holding
      (Variables|Grabbing|Current|SetbIsHoldingObject false)
      ;;[1 1 1] Move the crane up
      (Movement|ClampDestination (Math|Vector|MakeVector (.x _cranedestination) (.y _cranedestination) 0.0))
      (EventDispatchers|BindEventtoOnDestinationReached (EventDispatchers|CreateEvent :!event Custom|OnCraneFinishedGoingUp))
      ;[1 1 1] Play the detach sound
      (Audio|PlaySoundatLocation "/Game/VRPuzzle/Sectors/CargoBay/BeamCrane/Audio/A_Hiss_Cue.A_Hiss_Cue" (Transformation|GetWorldLocation (Variables|Default|GetCraneHeadPicker)) "0, 0, 0" 1.0 1.0 0.0 0 0 0 0))))

(event Custom|ChangeCraneDestination
  (params (DeltaX :type Float%20%28double-precision%29) (DeltaY :type Float%20%28double-precision%29))
  ;[1 1 1] Try to move the crane destination
  (if (Variables|Movement|GetbCanBeControlled)
    (Movement|ClampDestination (+ (Math|Vector|MakeVector DeltaX DeltaY 0.0) (Variables|Movement|GetCraneDestination)))))

(event Custom|GrabbableReached
  (bind _targetgrabbableactor (Variables|Grabbing|Current|GetTargetGrabbableActor))
  (bind _cranedestination (Variables|Movement|GetCraneDestination))
  ;[0.3083 0.3895 1] Grab the object when we reach it after grabbing
  (EventDispatchers|UnbindEventfromOnDestinationReached (delegate Custom|GrabbableReached))
  (Utilities|IsValid _targetgrabbableactor
    (:Is%20Valid
      (Utilities|FlowControl|Sequence
        (:then_0
          (bind _grabpointcomponent (Class|BPICraneGrabbable|TryGetGrabPointComponent(Message) _targetgrabbableactor)))
        (:then_1
          (bind (_extents _grabpointoffset) (Class|BPICraneGrabbable|TryGetExtents(Message) _targetgrabbableactor))
          (Grabbing|AttachGrabbable _grabpointcomponent _extents _grabpointoffset)
          ;[1 1 1] Move the crane fully up
          (Movement|ClampDestination (Math|Vector|MakeVector (.x _cranedestination) (.y _cranedestination) 0.0))
          (EventDispatchers|BindEventtoOnDestinationReached (EventDispatchers|CreateEvent :!event Custom|OnCraneFinishedGoingUp)))))))

(event Custom|OnCraneFinishedGoingUp
  ;[1 1 1] Re-enable controls when crane reaches top
  (EventDispatchers|UnbindEventfromOnDestinationReached (delegate Custom|OnCraneFinishedGoingUp))
  (Variables|Movement|SetbCanBeControlled true))

(event Custom|TryGrabbingOrReleasing
  ;[1 1 1] Try Grab/Release
  (if (Variables|Movement|GetbCanBeControlled)
    (if (Variables|Grabbing|Current|GetbIsHoldingObject)
      (bind (_bcanplacegrabbable _placepoint) (Grabbing|CheckifCanPlaceGrabbable))
      (if _bcanplacegrabbable
        (Grabbing|StartPlacingGrabbable _placepoint))
      (else
        (Grabbing|TryGrabGrabbable)))))

(event EventBeginPlay
  (bind _cranespaceendnear (Variables|Default|GetCraneSpaceEndNear))
  (bind _returnvalue (Transformation|GetWorldLocation _cranespaceendnear))
  ;[1 1 1] Calculate Allowed space
  (Variables|Movement|SetCraneSpaceDimensions (CallFunction|CalculateCraneSpace))
  ;[1 1 1] Calculate center point
  (bind _output_get (Variables|Movement|SetCraneCenterPoint (+ (/ (- (Transformation|GetWorldLocation (Variables|Default|GetCraneSpaceEndFar)) _returnvalue) (Math|Float|MakeLiteralFloat 2.0)) _returnvalue)))
  (Rendering|Debug|DrawDebugBox _output_get "300.000000,300.000000,300.000000" "(R=0.850279,G=0.337497,B=1.000000,A=1.000000)" "0, 0, 0" 1.0 2.0)
  ;[1 1 1] Calculate Z Offset of the head
  (Variables|Movement|SetCraneHeadPickerZOffset (.z (- (Variables|/Script/Engine.SceneComponent|GetRelativeLocation (Variables|Default|GetCraneMovementCenter)) (Variables|/Script/Engine.SceneComponent|GetRelativeLocation (Variables|Default|GetCraneHead)))))
  ;[0 0.07558 1] Move to center
  (Movement|ClampDestination "0, 0, 0")
  (Default|SetupCamera (Variables|Default|GetBP_CameraCapturerComponent) (Variables|Default|GetCraneCamera) "/Game/VRPuzzle/Sectors/CargoBay/BeamCrane/RT_CraneCamera.RT_CraneCamera"))

(event EventTick
  (params (DeltaSeconds :type Float%20%28single-precision%29))
  ;[1 1 1] Tick crane movement to destination
  (Movement|MoveCraneTick)
  (CallFunction|UpdateCraneServoSound))

(fn ConstructionScript
  (bind _cranespaceendfar (Variables|Default|GetCraneSpaceEndFar))
  (bind _cranespaceendnear (Variables|Default|GetCraneSpaceEndNear))
  (bind _relativelocation (Variables|/Script/Engine.SceneComponent|GetRelativeLocation _cranespaceendfar))
  (bind _relativelocation_2 (Variables|/Script/Engine.SceneComponent|GetRelativeLocation _cranespaceendnear))
  (bind _returnvalue (- _relativelocation _relativelocation_2))
  (bind _returnvalue_2 (Math|Vector|VectorGetAbs _returnvalue))
  (bind _cranemovementboundsvisualization (Variables|Default|GetCraneMovementBoundsVisualization)
    (:then
      (Transformation|SetRelativeScale3D _cranemovementboundsvisualization (Math|Conversions|ToVector(Vector2D) (Math|Conversions|ToVector2D(Vector) (/ _returnvalue_2 (Math|Float|MakeLiteralFloat 1e+02))))))
    (:else
      _))
  (Transformation|SetRelativeLocation (Variables|Default|GetCraneMovementCenter) (+ (/ _returnvalue_2 (Math|Float|MakeLiteralFloat 2.0)) (Variables|/Script/Engine.SceneComponent|GetRelativeLocation (Variables|Default|GetCraneSpaceEndNear))) false false))

(fn MoveCraneTick
  (bind _beams (Variables|Default|GetBeams))
  (bind _cranehead (Variables|Default|GetCraneHead))
  (bind _cranehead_2 (Variables|Default|GetCraneHead))
  (bind _craneheadpicker (Variables|Default|GetCraneHeadPicker))
  (bind _cranehead_3 (Variables|Default|GetCraneHead))
  (bind _cranehead_4 (Variables|Default|GetCraneHead))
  (bind _craneheadpicker_2 (Variables|Default|GetCraneHeadPicker))
  (bind _relativelocation (Variables|/Script/Engine.SceneComponent|GetRelativeLocation _craneheadpicker))
  (bind _relativelocation_2 (Variables|/Script/Engine.SceneComponent|GetRelativeLocation _cranehead))
  (bind _relativelocation_3 (Variables|/Script/Engine.SceneComponent|GetRelativeLocation _cranehead_3))
  (bind _relativelocation_4 (Variables|/Script/Engine.SceneComponent|GetRelativeLocation _cranehead_4))
  (bind _relativelocation_5 (Variables|/Script/Engine.SceneComponent|GetRelativeLocation _craneheadpicker_2))
  (bind _relativelocation_6 (Variables|/Script/Engine.SceneComponent|GetRelativeLocation _beams))
  (LocalVariables|SetLastPosition (Math|Vector|MakeVector (.x _relativelocation_2) (.y _relativelocation_2) (- (.z (Variables|/Script/Engine.SceneComponent|GetRelativeLocation (Variables|Default|GetCraneHeadPicker))) (Variables|Movement|GetCraneHeadPickerZOffset))))
  ;[0.02788 1 0] Calculate the new Y location in local space
  (LocalVariables|SetCurrentDifferenceY (- (.y (Variables|Movement|GetCraneDestination)) (.y _relativelocation_3)))
  (LocalVariables|SetNewY (Math|Interpolation|FInterptoConstant (.y _relativelocation_3) (.y (Variables|Movement|GetCraneDestination)) (Utilities|Time|GetWorldDeltaSeconds) (.y (Variables|Movement|GetCraneMovementSpeed))))
  ;[1 0.05824 0] Calculate the new X location in local space
  (LocalVariables|SetCurrentDifferenceX (- (.x (Variables|Movement|GetCraneDestination)) (.x _relativelocation_4)))
  (LocalVariables|SetNewX (Math|Interpolation|FInterptoConstant (.x _relativelocation_4) (.x (Variables|Movement|GetCraneDestination)) (Utilities|Time|GetWorldDeltaSeconds) (.x (Variables|Movement|GetCraneMovementSpeed))))
  ;[0 0.119 1] Calculate the new Z location in local space
  (LocalVariables|SetCurrentDifferenceZ (- (+ (.z (Variables|Movement|GetCraneDestination)) (Variables|Movement|GetCraneHeadPickerZOffset)) (.z _relativelocation_5)))
  (LocalVariables|SetNewZ (Math|Interpolation|FInterptoConstant (.z _relativelocation_5) (+ (.z (Variables|Movement|GetCraneDestination)) (Variables|Movement|GetCraneHeadPickerZOffset)) (Utilities|Time|GetWorldDeltaSeconds) (.z (Variables|Movement|GetCraneMovementSpeed))))
  (if (Variables|Grabbing|Current|GetbIsHoldingObject)
    ;[1 1 1] If holding anything, check if can move
    (bind _canmove (Movement|CheckifMovePossible (Math|Vector|MakeVector (LocalVariables|GetCurrentDifferenceX) (LocalVariables|GetCurrentDifferenceY) (LocalVariables|GetCurrentDifferenceZ))))
    (if _canmove
      _
      (else
        (Variables|Movement|SetCraneDestination (- (Variables|Movement|GetCraneDestination) (Math|Vector|MakeVector (LocalVariables|GetCurrentDifferenceX) (LocalVariables|GetCurrentDifferenceY) (LocalVariables|GetCurrentDifferenceZ))))
        (Variables|Movement|SetLastTickMovement "0, 0, 0")
        (return))))
  (Variables|Movement|SetLastTickMovement (- (Math|Vector|MakeVector (LocalVariables|GetNewX) (LocalVariables|GetNewY) (- (LocalVariables|GetNewZ) (Variables|Movement|GetCraneHeadPickerZOffset))) (LocalVariables|GetLastPosition)))
  ;[0.1067 1 0.1313 0.199 36] Move Crane
  (Utilities|FlowControl|Sequence
    (:then_0
      ;;[1 1 1] Set beams location
      (Transformation|SetRelativeLocation _beams (Math|Vector|MakeVector (.x _relativelocation_6) (LocalVariables|GetNewY) (.z _relativelocation_6)) false false))
    (:then_1
      ;;[1 1 1] Set Head location
      (Transformation|SetRelativeLocation _cranehead_2 (Math|Vector|MakeVector (LocalVariables|GetNewX) (LocalVariables|GetNewY) (.z (Variables|/Script/Engine.SceneComponent|GetRelativeLocation _cranehead_2))) false false))
    (:then_2
      ;;[1 1 1] Set Head Picker location
      (Transformation|SetRelativeLocation _craneheadpicker (Math|Vector|MakeVector (.x _relativelocation) (.y _relativelocation) (LocalVariables|GetNewZ)) false false))
    (:then_3
      ;;[1 0.7427 0.9925] Trigger the destination reached event, but only once per destination
      (if (not (Variables|Movement|GetbHasReachedCurrentDestination))
        (if (<= (Math|Vector|VectorLength (Math|Vector|MakeVector (LocalVariables|GetCurrentDifferenceX) (LocalVariables|GetCurrentDifferenceY) (LocalVariables|GetCurrentDifferenceZ))) 5.0)
          (Variables|Movement|SetbHasReachedCurrentDestination true)
          (Default|CallOnDestinationReached))))))

(fn ClampDestination
  (params (NewDestination :type Vector))
  (bind _returnvalue (Math|Float|MakeLiteralFloat 2.0))
  (bind _cranespacedimensions (Variables|Movement|GetCraneSpaceDimensions))
  (bind _returnvalue_2 (/ _cranespacedimensions _returnvalue))
  (bind _returnvalue_3 (Class|KismetMathLibrary|Negated2D _returnvalue_2))
  (bind (_x _y) (Math|Vector2D|BreakVector2D _returnvalue_2))
  (Variables|Movement|SetCraneDestination (Math|Vector|MakeVector (Math|Float|Clamp(Float) (.x NewDestination) (.x _returnvalue_3) _x) (Math|Float|Clamp(Float) (.y NewDestination) (.y _returnvalue_3) _y) (Math|Float|Min(Float) (.z NewDestination) (- (Variables|Movement|GetCraneHeadPickerMin) (Variables|Movement|GetCraneHeadPickerZOffset)))))
  (Variables|Movement|SetbHasReachedCurrentDestination false)
  (return))

(fn TryGrabGrabbable
  (bind _craneheadpicker (Variables|Default|GetCraneHeadPicker))
  (bind _returnvalue (Transformation|GetWorldLocation _craneheadpicker))
  (if (Variables|Grabbing|Current|GetbIsHoldingObject)
    ;[1 1 1] Already holding an object
    (return)
    (else
      ;[0.7528 0.6665 1] Check if anything to grab below
      (bind (_outhit _returnvalue_2) (Collision|BoxTraceByChannel _returnvalue (+ _returnvalue (* (Math|Vector|GetUpVector (Variables|Default|GetCraneHeadPicker)) (* (Variables|Grabbing|Settings|GetGrabMaxDistance) -1.0))) (Variables|Grabbing|Settings|GetGrabPrecision) (Transformation|GetWorldRotation (Variables|Default|GetDefaultSceneRoot)) "TraceTypeQuery1" false 0 "ForDuration"))
      (if _returnvalue_2
        (bind _output_get (LocalVariables|SetTraceResults _outhit))
        (bind _bcanbegrabbed (Class|BPICraneGrabbable|GetCanbeGrabbed(Message) (.HitActor (Collision|BreakHitResult _output_get))))
        (if _bcanbegrabbed
          (bind _bcanpickupgrabbable (Grabbing|CheckifCanGrabGrabbable (.HitActor (Collision|BreakHitResult _output_get))))
          (if _bcanpickupgrabbable
            (bind _grabpointcomponent (Class|BPICraneGrabbable|TryGetGrabPointComponent(Message) (.HitActor (Collision|BreakHitResult _output_get))))
            (Grabbing|StartGrab _grabpointcomponent)
            (Variables|Grabbing|Current|SetTargetGrabbableActor (.HitActor (Collision|BreakHitResult _output_get)))
            (Variables|Movement|SetbCanBeControlled false)
            (return)
            (else
              (return)))
          (else
            ;[1 1 1] Hit object is not grabbable
            (return)))
        (else
          ;[1 1 1] Nothing to grab
          (return))))))

(fn AttachGrabbable
  (params (GrabPointComponent :type Primitive%20Component%20Object%20Reference) (Extents :type Vector) (GrabPointOffset :type Vector))
  (bind _output_get (LocalVariables|SetGrabbableActor (Components|GetOwner GrabPointComponent)))
  ;[1 1 1] Debug Display the name of the grabbed object
  (Development|PrintString (Utilities|String|Append "Grabbing " (Utilities|GetDisplayName _output_get)))
  ;[1 1 1] Attach to grab socket
  (Transformation|AttachComponentToComponent (LocalVariables|GetGrabbableActor) (Variables|Default|GetCraneHeadPicker) "CraneAttachPoint" "SnapToTarget" "KeepWorld" "KeepRelative" true)
  ;[1 1 1] Offset so the grab point is on the socket
  (Transformation|AddActorLocalOffset (LocalVariables|GetGrabbableActor) (Math|Vector|NegateVector GrabPointOffset) false false)
  (Class|BPICraneGrabbable|SetCollisionStatus(Message) (LocalVariables|GetGrabbableActor) false)
  (Variables|Grabbing|Current|SetCurrentGrabbableExtents Extents)
  (Variables|Grabbing|Current|SetCurrentGrabbablePointOffset (Variables|Grabbing|Current|GetCurrentGrabbablePointOffset))
  (Variables|Grabbing|Current|SetbIsHoldingObject true)
  ;[1 1 1] Play the attach sound
  (Audio|PlaySoundatLocation "/Game/VRPuzzle/Sectors/CargoBay/BeamCrane/Audio/A_Hiss_Cue.A_Hiss_Cue" (Transformation|GetWorldLocation (Variables|Default|GetCraneHeadPicker)) "0, 0, 0" 1.0 1.0 0.0 0 0 0 0)
  (return))

(fn StartGrab
  (params (GrabPointComponent :type Primitive%20Component%20Object%20Reference))
  (bind _returnvalue (Movement|ProjecttoCranePlane (Transformation|GetWorldLocation GrabPointComponent)))
  (Movement|ClampDestination _returnvalue)
  ;[1 1 1] Handle the grabbing when we reach the object
  (EventDispatchers|BindEventtoOnDestinationReached (EventDispatchers|CreateEvent :!event Custom|GrabbableReached))
  (return))

(fn ProjecttoCranePlane
  (params (Point :type Vector))
  (bind _cranehead (Variables|Default|GetCraneHead))
  (bind _cranecenterpoint (Variables|Movement|GetCraneCenterPoint))
  (bind _returnvalue (Math|Vector|GetUpVector _cranehead))
  (bind _returnvalue_2 (Math|Vector|NegateVector _returnvalue))
  (bind _returnvalue_3 (Class|KismetMathLibrary|ProjectPointontoPlane Point _cranecenterpoint _returnvalue_2))
  (bind (_x _y) (Math|Vector|BreakVector _returnvalue_3))
  (return (* (Math|Vector|RotateVector (- (Transformation|GetWorldLocation (Variables|Default|GetCraneMovementCenter)) (Math|Vector|MakeVector _x _y (.Z (Math|Vector|BreakVector Point)))) (Transformation|GetActorRotation)) "1.000000,1.000000,-1.000000")))

(fn CheckifCanPlaceGrabbable
  (bind _craneheadpicker (Variables|Default|GetCraneHeadPicker))
  (bind _currentgrabbableextents (Variables|Grabbing|Current|GetCurrentGrabbableExtents))
  (bind _returnvalue (* _currentgrabbableextents "0.000000,0.000000,1.000000"))
  ;[1 1 1] Get the lowest point cast from the center of the crane
  (bind (_outhit _returnvalue_2) (Collision|BoxTraceByChannel (- (Transformation|GetWorldLocation (Variables|Default|GetCraneHeadPicker)) (* (Variables|Grabbing|Current|GetCurrentGrabbableExtents) "0.000000,0.000000,1.000000")) (+ (Transformation|GetWorldLocation _craneheadpicker) (* (Math|Vector|NegateVector (Math|Vector|GetUpVector _craneheadpicker)) (Variables|Grabbing|Settings|GetGrabMaxDistance))) "25.000000,25.000000,1.000000" "0, 0, 0" "TraceTypeQuery1" false 0 "ForDuration"))
  (if _returnvalue_2
    (LocalVariables|SetLowerHitPoint (.Location (Collision|BreakHitResult _outhit)))
    ;[1 1 1] Try trace the entire grabbable down
    (bind _returnvalue_3 (Collision|BoxTraceByChannel (- (Transformation|GetWorldLocation (Variables|Default|GetCraneHeadPicker)) _returnvalue) (+ (LocalVariables|GetLowerHitPoint) "0.000000,0.000000,5.000000" _returnvalue) (Variables|Grabbing|Current|GetCurrentGrabbableExtents) (Transformation|GetActorRotation (Variables|Grabbing|Current|GetTargetGrabbableActor)) "TraceTypeQuery1" false 0 "ForDuration" true "(R=0.805426,G=0.350314,B=1.000000,A=1.000000)" "(R=0.339465,G=1.000000,B=0.582165,A=1.000000)" 2.0))
    ;[1 1 1] Check if no hits on the way down
    (if _returnvalue_3
      (return false "0, 0, 0")
      (else
        ;[1 1 1] Can place, return hit point
        (return true (LocalVariables|GetLowerHitPoint))))
    (else
      (return false "0, 0, 0"))))

(fn StartPlacingGrabbable
  (params (PlacePoint :type Vector))
  (bind _returnvalue (Movement|ProjecttoCranePlane (Math|Vector|MakeVector (.x PlacePoint) (.y PlacePoint) (+ (.z PlacePoint) (* (.z (Variables|Grabbing|Current|GetCurrentGrabbableExtents)) 2.0) (.z (Variables|Grabbing|Current|GetCurrentGrabbablePointOffset))))))
  (Movement|ClampDestination _returnvalue)
  (Variables|Movement|SetbCanBeControlled false)
  (EventDispatchers|BindEventtoOnDestinationReached (EventDispatchers|CreateEvent :!event Custom|PlaceLocationReached))
  (return))

(fn CalculateCraneSpace
  (return (Math|Conversions|ToVector2D(Vector) (Math|Vector|VectorGetAbs (- (Variables|/Script/Engine.SceneComponent|GetRelativeLocation (Variables|Default|GetCraneSpaceEndFar)) (Variables|/Script/Engine.SceneComponent|GetRelativeLocation (Variables|Default|GetCraneSpaceEndNear)))))))

(fn CheckifCanGrabGrabbable
  (params (GrabbableActor :type Actor%20Object%20Reference))
  (bind _returnvalue (Transformation|GetActorLocation GrabbableActor))
  (bind _grabpointcomponent (Class|BPICraneGrabbable|TryGetGrabPointComponent(Message) GrabbableActor))
  (LocalVariables|SetGrabPoint _grabpointcomponent)
  (bind _extents (Class|BPICraneGrabbable|TryGetExtents(Message) GrabbableActor))
  ;[1 1 1] Try trace the entire grabbable up
  (bind _returnvalue_2 (Collision|BoxTraceByChannel (- (Math|Vector|MakeVector (.x _returnvalue) (.y _returnvalue) (.z (Transformation|GetWorldLocation (Variables|Default|GetCraneHeadPicker)))) (* _extents "0.000000,0.000000,1.000000")) (+ (* _extents "0.000000,0.000000,1.000000") "0.000000,0.000000,5.000000" (Transformation|GetActorLocation GrabbableActor)) _extents (Transformation|GetActorRotation GrabbableActor) "TraceTypeQuery1" false (Utilities|Array|MakeArray GrabbableActor) "ForDuration" true "(R=0.805426,G=0.350314,B=1.000000,A=1.000000)" "(R=0.339465,G=1.000000,B=0.582165,A=1.000000)" 2.0))
  ;[1 1 1] Check if no hits on the way down
  (if _returnvalue_2
    (return false)
    (else
      ;[1 1 1] Can place, return hit point
      (return true))))

(fn CheckifMovePossible
  (params (CraneRelativeLocationDifference :type Vector))
  (bind _returnvalue (Transformation|GetActorRotation))
  (bind _craneheadpicker (Variables|Default|GetCraneHeadPicker))
  (bind _currentgrabbableextents (Variables|Grabbing|Current|GetCurrentGrabbableExtents))
  (bind _returnvalue_2 (Transformation|GetWorldLocation _craneheadpicker))
  (bind _returnvalue_3 (Math|Vector|RotateVector CraneRelativeLocationDifference _returnvalue))
  (bind _returnvalue_4 (* _currentgrabbableextents "0.000000,0.000000,1.000000"))
  (bind _returnvalue_5 (- _returnvalue_2 _returnvalue_4))
  (bind _returnvalue_6 (+ _returnvalue_5 "0.000000,0.000000,25.000000" _returnvalue_3))
  ;[1 1 1] Check for any hits in the predicted position
  (bind _returnvalue_7 (Collision|BoxTraceByChannel _returnvalue_6 _returnvalue_6 (Variables|Grabbing|Current|GetCurrentGrabbableExtents) (Transformation|GetActorRotation (Variables|Grabbing|Current|GetTargetGrabbableActor)) "TraceTypeQuery1" false (Utilities|Array|MakeArray (Variables|Grabbing|Current|GetTargetGrabbableActor)) "ForOneFrame" true "(R=0.972238,G=0.000000,B=1.000000,A=1.000000)" "(R=0.000000,G=0.974876,B=1.000000,A=1.000000)"))
  (return (not _returnvalue_7)))

(fn UpdateCraneServoSound
  (bind _output_get (Variables|Movement|Audio|SetLastVolumeMultiplier (Math|Interpolation|FInterpTo (Variables|Movement|Audio|GetLastVolumeMultiplier) (Math|Curves|GetFloatValue (Variables|Movement|Audio|GetServoVolumeCurve) (Math|Vector|VectorLength (Variables|Movement|GetLastTickMovement))) (Utilities|Time|GetWorldDeltaSeconds) (Variables|Movement|Audio|GetVolumeMultiplierMaxChange))))
  (Audio|Components|Audio|SetVolumeMultiplier (Variables|Default|GetCraneAudioSource) _output_get :!class /Script/Engine.AudioComponent))