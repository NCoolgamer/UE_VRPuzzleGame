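; BP_LaserEmitter is a laser emitter for the cargo bay beam crane, drawing its beam with a Niagara effect.
; Each tick it line-traces the Visibility channel along the effect's forward vector between minimum and maximum distances.
; The hit point, or maximum range when nothing is hit, sets the beam's end location.
; SetLaserEnabledState toggles both the effect and ticking, so a disabled laser stops tracing.
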(event EventTick
  (params (DeltaSeconds :type Float%20%28single-precision%29))
  (bind (_outhit _returnvalue) (Collision|LineTraceByChannel (+ (Transformation|GetActorLocation) (* (Math|Vector|GetForwardVector (Variables|Default|GetNS_CraneLaser)) (Variables|Default|GetMinDistance))) (+ (Transformation|GetActorLocation) (* (Math|Vector|GetForwardVector (Variables|Default|GetNS_CraneLaser)) (Variables|Default|GetMaxDistance))) "TraceTypeQuery1" false 0 "None"))
  (Niagara|SetNiagaraVariable(Vector3) (Variables|Default|GetNS_CraneLaser) "LaserEndLocation" (Math|Vector|SelectVector (.Location (Collision|BreakHitResult _outhit)) (+ (Transformation|GetActorLocation) (* (Math|Vector|GetForwardVector (Variables|Default|GetNS_CraneLaser)) (Variables|Default|GetMaxDistance))) _returnvalue)))

(event EventSetLaserEnabledState
  (params (bEnable :type Boolean))
  (Components|Activation|SetActive (Variables|Default|GetNS_CraneLaser) bEnable true)
  (Actor|Tick|SetActorTickEnabled bEnable))

(fn ConstructionScript)