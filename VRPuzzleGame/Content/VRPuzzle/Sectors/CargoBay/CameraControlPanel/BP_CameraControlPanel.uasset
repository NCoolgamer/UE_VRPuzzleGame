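; CCTV control panel for the VR puzzle's Cargo Bay that lets the player cycle through and rotate security cameras while unlocked by a keycard.
; Receiver events from the child keycard reader toggle the panel, disabling it once no valid senders remain.
; Child pushable buttons switch cameras on press and rotate them while held, or play a throttled error sound when locked.
; Only the selected camera captures, and disabling draws a locked-screen material to the render target.
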(event Custom|SwitchToNextCamera
  (bind _currentcameraindex (Variables|Default|GetCurrentCameraIndex))
  (bind _returnvalue (+ _currentcameraindex 1))
  ;[1 1 1] Camera switching
  (if (Variables|Default|GetbIsEnabled)
    (if (< _returnvalue (Utilities|Array|Length (Variables|Default|GetCameraList)))
      (CallFunction|SwitchtoCamerabyIndex _returnvalue)
      (else
        (CallFunction|SwitchtoCamerabyIndex)))
    (else
      (CallFunction|PlayErrorSound))))

(event Custom|SwitchToPreviousCamera
  (bind _currentcameraindex (Variables|Default|GetCurrentCameraIndex))
  (bind _returnvalue (+ _currentcameraindex -1))
  ;[1 1 1] Camera switching
  (if (Variables|Default|GetbIsEnabled)
    (if (>= _returnvalue 0)
      (CallFunction|SwitchtoCamerabyIndex _returnvalue)
      (else
        (CallFunction|SwitchtoCamerabyIndex (- (Utilities|Array|Length (Variables|Default|GetCameraList)) 1))))
    (else
      (CallFunction|PlayErrorSound))))

(event Custom|RotateLButtonTick
  ;[1 1 1] Handle camera rotation buttons
  (if (Variables|Default|GetbIsEnabled)
    (Default|RotateCameraLeftTick (Utilities|Array|Get(acopy) (Variables|Default|GetCameraList) (Variables|Default|GetCurrentCameraIndex)))
    (else
      (CallFunction|PlayErrorSound))))

(event Custom|RotateRButtonTick
  ;[1 1 1] Handle camera rotation buttons
  (if (Variables|Default|GetbIsEnabled)
    (Default|RotateCameraRightTick (Utilities|Array|Get(acopy) (Variables|Default|GetCameraList) (Variables|Default|GetCurrentCameraIndex)))
    (else
      (CallFunction|PlayErrorSound))))

(event Custom|DisablePanel
  (CallFunction|SwitchPanelEnabledState false)
  (Development|PrintString "Disabling CCTV Panel"))

(event Custom|EnablePanel
  (CallFunction|SwitchPanelEnabledState true)
  (Development|PrintString "Enabling CCTV Panel")
  (Audio|PlaySoundatLocation "/Game/VRPuzzle/Sectors/CargoBay/CameraControlPanel/Audio/A_PanelEnabled_Cue.A_PanelEnabled_Cue" (Transformation|GetActorLocation) "0, 0, 0" 1.0 1.0 0.0 0 0 0 0))

(event Custom|PlayErrorSound
  (Utilities|FlowControl|DoOnce false :!label _label
    (:Completed
      (Audio|PlaySoundatLocation "/Game/VRPuzzle/Sectors/CargoBay/CameraControlPanel/Audio/A_PanelError_Cue.A_PanelError_Cue" (Transformation|GetActorLocation) "0, 0, 0" 1.0 1.0 0.0 0 0 0 0)
      (Utilities|FlowControl|Delay 1.0)
      (goto _label Reset))))

(event Custom|CheckIfShouldDisablePanel
  (params (ValidSendersLeft :type Integer))
  ;[1 1 1] Setup Keycard reader
  (if (<= ValidSendersLeft 0)
    (CallFunction|DisablePanel)))

(event EventBeginPlay
  (bind _bp_keycardreader (Variables|Default|GetBP_KeycardReader))
  (bind _childactor (Variables|/Script/Engine.ChildActorComponent|GetChildActor _bp_keycardreader))
  (bind _returnvalue (Actor|GetComponentbyClass _childactor "/Game/VRPuzzle/Core/Interactables/NearFieldInteraction/BP_NFReceiverComponent.BP_NFReceiverComponent_C"))
  (CallFunction|SwitchPanelEnabledState false)
  (CallFunction|SetupCameraSwitchButtons)
  (CallFunction|SetupCameraRotationButtons)
  ;[1 1 1] Setup Keycard reader
  (EventDispatchers|BindEventtoOnValidSenderBeginOverlap _returnvalue (EventDispatchers|CreateEvent :!event Custom|EnablePanel))
  (EventDispatchers|BindEventtoOnValidSenderEndOverlap _returnvalue (delegate Custom|CheckIfShouldDisablePanel)))

(fn ConstructionScript)

(fn SetupCameraSwitchButtons
  (Utilities|FlowControl|Sequence
    (:then_0
      (bind _asbp_pushable_button (Utilities|Casting|CastToBP_PushableButton (Variables|/Script/Engine.ChildActorComponent|GetChildActor (Variables|Default|GetNextCameraButton))))
      (EventDispatchers|BindEventtoOnButtonPressed _asbp_pushable_button (EventDispatchers|CreateEvent :!event Custom|SwitchToNextCamera)))
    (:then_1
      (bind _asbp_pushable_button_2 (Utilities|Casting|CastToBP_PushableButton (Variables|/Script/Engine.ChildActorComponent|GetChildActor (Variables|Default|GetPreviousCameraButton))))
      (EventDispatchers|BindEventtoOnButtonPressed _asbp_pushable_button_2 (EventDispatchers|CreateEvent :!event Custom|SwitchToPreviousCamera))
      (return))))

(fn SwitchtoCamerabyIndex
  (params (NewIndex :type Integer))
  ;[1 1 1] Stop old camera
  (Default|StopCapturing (Variables|/Game/VRPuzzle/Sectors/CargoBay/CameraControlPanel/BP_SecurityCamera.BP_SecurityCamera_C|GetBP_CameraCapturerComponent (Utilities|Array|Get(acopy) (Variables|Default|GetCameraList) (Variables|Default|GetCurrentCameraIndex))))
  ;[1 1 1] Start new camera
  (Default|StartCapturing (Variables|/Game/VRPuzzle/Sectors/CargoBay/CameraControlPanel/BP_SecurityCamera.BP_SecurityCamera_C|GetBP_CameraCapturerComponent (Utilities|Array|Get(acopy) (Variables|Default|GetCameraList) NewIndex)))
  (Variables|Default|SetCurrentCameraIndex NewIndex))

(fn SetupCameraRotationButtons
  (Utilities|FlowControl|Sequence
    (:then_0
      (bind _asbp_pushable_button (Utilities|Casting|CastToBP_PushableButton (Variables|/Script/Engine.ChildActorComponent|GetChildActor (Variables|Default|GetRotateRButton))))
      (EventDispatchers|BindEventtoOnButtonHeldTick _asbp_pushable_button (EventDispatchers|CreateEvent :!event Custom|RotateRButtonTick)))
    (:then_1
      (bind _asbp_pushable_button_2 (Utilities|Casting|CastToBP_PushableButton (Variables|/Script/Engine.ChildActorComponent|GetChildActor (Variables|Default|GetRotateLButton))))
      (EventDispatchers|BindEventtoOnButtonHeldTick _asbp_pushable_button_2 (EventDispatchers|CreateEvent :!event Custom|RotateLButtonTick)))))

(fn SwitchPanelEnabledState
  (params (bShouldEnable :type Boolean))
  (if bShouldEnable
    ;[1 1 1] Enable Controls
    (Variables|Default|SetbIsEnabled true)
    ;[1 1 1] Start drawing the camera
    (Default|StartCapturing (Variables|/Game/VRPuzzle/Sectors/CargoBay/CameraControlPanel/BP_SecurityCamera.BP_SecurityCamera_C|GetBP_CameraCapturerComponent (Utilities|Array|Get(acopy) (Variables|Default|GetCameraList) (Variables|Default|GetCurrentCameraIndex))))
    (else
      ;[1 1 1] Disable Controls
      (Variables|Default|SetbIsEnabled false)
      ;[1 1 1] Stop drawing the camera
      (Default|StopCapturing (Variables|/Game/VRPuzzle/Sectors/CargoBay/CameraControlPanel/BP_SecurityCamera.BP_SecurityCamera_C|GetBP_CameraCapturerComponent (Utilities|Array|Get(acopy) (Variables|Default|GetCameraList) (Variables|Default|GetCurrentCameraIndex))))
      ;[1 1 1] Draw locked texture
      (Rendering|DrawMaterialtoRenderTarget "/Game/VRPuzzle/Sectors/CargoBay/CameraControlPanel/RT_SecurityCamera.RT_SecurityCamera" "/Game/VRPuzzle/Sectors/CargoBay/CameraControlPanel/M_LockedScreen.M_LockedScreen"))))