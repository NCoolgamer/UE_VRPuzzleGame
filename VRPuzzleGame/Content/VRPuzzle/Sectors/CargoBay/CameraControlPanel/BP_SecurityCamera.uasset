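; BP_SecurityCamera is a rotatable security camera in the VR puzzle's cargo bay that captures its view to a render target.
; On BeginPlay it applies the start yaw and hands its scene capture and render target to BPCameraCapturerComponent.
; Externally triggered left and right tick events move the pivot's yaw at constant speed toward the rotation bounds, so the actor's own Tick stays unused.
; The construction script also applies the start yaw.
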(event Custom|RotateCameraTick
  (params (bRotateRight :type Boolean))
  (CallFunction|SetCameraRotation (Math|Float|SelectFloat (Math|Interpolation|FInterptoConstant (.yaw (Variables|/Script/Engine.SceneComponent|GetRelativeRotation (Variables|Default|GetCameraRotationPivot))) (.y (Variables|Default|GetRotationBounds)) (Utilities|Time|GetWorldDeltaSeconds) (Variables|Default|GetCameraRotationSpeed)) (Math|Interpolation|FInterptoConstant (.yaw (Variables|/Script/Engine.SceneComponent|GetRelativeRotation (Variables|Default|GetCameraRotationPivot))) (.x (Variables|Default|GetRotationBounds)) (Utilities|Time|GetWorldDeltaSeconds) (Variables|Default|GetCameraRotationSpeed)) bRotateRight)))

(event Custom|RotateCameraRightTick
  (CallFunction|RotateCameraTick true))

(event Custom|RotateCameraLeftTick
  (CallFunction|RotateCameraTick false))

(event EventBeginPlay
  (CallFunction|SetCameraRotation (Variables|Default|GetStartRotation))
  (Default|SetupCamera (Variables|Default|GetBP_CameraCapturerComponent) (Variables|Default|GetCameraCapturer) "/Game/VRPuzzle/Sectors/CargoBay/CameraControlPanel/RT_SecurityCamera.RT_SecurityCamera"))

(event Collision|EventActorBeginOverlap
  (params (OtherActor :type Actor%20Object%20Reference)))

(event EventTick
  (params (DeltaSeconds :type Float%20%28single-precision%29)))

(fn ConstructionScript
  (CallFunction|SetCameraRotation (Variables|Default|GetStartRotation)))

(fn SetCameraRotation
  (params (NewRotation_Yaw :type Float%20%28single-precision%29))
  (bind _camerarotationpivot (Variables|Default|GetCameraRotationPivot))
  (bind _relativerotation (Variables|/Script/Engine.SceneComponent|GetRelativeRotation _camerarotationpivot))
  (Transformation|SetRelativeRotation (Variables|Default|GetCameraRotationPivot) (Math|Rotator|MakeRotator (.roll _relativerotation) (.pitch _relativerotation) NewRotation_Yaw) false false))