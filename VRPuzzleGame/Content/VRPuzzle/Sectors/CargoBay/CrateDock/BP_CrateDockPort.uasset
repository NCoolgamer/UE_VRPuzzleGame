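; Cargo bay crate dock port with a sliding door, a spotlight and a status screen for the VR puzzle.
; Open and close events move the door by chaining next-tick timers that interpolate it between open and closed markers, then fire opened/closed dispatchers.
; Opening plays a pneumatic sound, and the light switches on once fully open and off when closing starts.
; Wrapper functions push dock name, status, docking progress and crate number to the screen widget.
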(event Custom|TickDoorClose
  ;[1 0.2904 0.2705 1 36] Close door
  (Transformation|SetRelativeLocation (Variables|Default|GetS_DockDoor) (Math|Interpolation|VInterpTo (Variables|/Script/Engine.SceneComponent|GetRelativeLocation (Variables|Default|GetS_DockDoor)) (Variables|/Script/Engine.SceneComponent|GetRelativeLocation (Variables|Default|GetDoorPositionClosed)) (Utilities|Time|GetWorldDeltaSeconds) (Variables|Default|GetDoorMovementSpeed)) false false)
  (if (Utilities|Operators|EqualEqual (Variables|/Script/Engine.SceneComponent|GetRelativeLocation (Variables|Default|GetS_DockDoor)) (Variables|/Script/Engine.SceneComponent|GetRelativeLocation (Variables|Default|GetDoorPositionClosed)) 5.0)
    (Variables|Default|SetbDoorIsOpen false)
    (Default|CallOnDoorClosed)
    (Variables|Default|SetDoorTickTimer "")
    (Development|PrintString "Cargo Door Closed")
    (else
      (bind _returnvalue (Class|KismetSystemLibrary|SetTimerforNextTickDelegate (EventDispatchers|CreateEvent :!event Custom|TickDoorClose)))
      (Variables|Default|SetDoorTickTimer _returnvalue))))

(event Custom|TickDoorOpen
  ;[0.1377 1 0.1279 1 36] Open door
  (Transformation|SetRelativeLocation (Variables|Default|GetS_DockDoor) (Math|Interpolation|VInterpTo (Variables|/Script/Engine.SceneComponent|GetRelativeLocation (Variables|Default|GetS_DockDoor)) (Variables|/Script/Engine.SceneComponent|GetRelativeLocation (Variables|Default|GetDoorPositionOpen)) (Utilities|Time|GetWorldDeltaSeconds) (Variables|Default|GetDoorMovementSpeed)) false false)
  (if (Utilities|Operators|EqualEqual (Variables|/Script/Engine.SceneComponent|GetRelativeLocation (Variables|Default|GetS_DockDoor)) (Variables|/Script/Engine.SceneComponent|GetRelativeLocation (Variables|Default|GetDoorPositionOpen)) 5.0)
    (Variables|Default|SetbDoorIsOpen true)
    (Default|CallOnDoorOpened)
    (Variables|Default|SetDoorTickTimer "")
    (Development|PrintString "Cargo Door Opened")
    (else
      (bind _returnvalue (Class|KismetSystemLibrary|SetTimerforNextTickDelegate (EventDispatchers|CreateEvent :!event Custom|TickDoorOpen)))
      (Variables|Default|SetDoorTickTimer _returnvalue))))

(event Custom|StartClosingDoor
  (if (Utilities|Time|IsValidTimerHandle (Variables|Default|GetDoorTickTimer))
    (Utilities|Time|ClearandInvalidateTimerbyHandle (Variables|Default|GetDoorTickTimer)))
  (bind _returnvalue (Class|KismetSystemLibrary|SetTimerforNextTickDelegate (EventDispatchers|CreateEvent :!event Custom|TickDoorClose)))
  (Variables|Default|SetDoorTickTimer _returnvalue)
  ;[1 1 1] Turn off light
  (Rendering|SetVisibility (Variables|Default|GetSpotLight) false false))

(event Custom|StartOpeningDoor
  (Audio|PlaySoundatLocation "/Game/VRPuzzle/Sectors/CargoBay/CrateDock/Audio/A_PneumaticDoor_Cue.A_PneumaticDoor_Cue" (Transformation|GetWorldLocation (Variables|Default|GetS_DockDoor)) "0, 0, 0" 1.0 1.0 0.0 0 0 0 0)
  (Utilities|FlowControl|Delay 0.5)
  (if (Utilities|Time|IsValidTimerHandle (Variables|Default|GetDoorTickTimer))
    (Utilities|Time|ClearandInvalidateTimerbyHandle (Variables|Default|GetDoorTickTimer)))
  (bind _returnvalue (Class|KismetSystemLibrary|SetTimerforNextTickDelegate (EventDispatchers|CreateEvent :!event Custom|TickDoorOpen)))
  (Variables|Default|SetDoorTickTimer _returnvalue))

(event Custom|TurnDoorLightOn
  ;[1 1 1] Bind light to door
  (Rendering|SetVisibility (Variables|Default|GetSpotLight) true false))

(event EventBeginPlay
  (CallFunction|UpdateDockScreenStatus)
  (CallFunction|SetDockName)
  (Transformation|SetRelativeLocation (Variables|Default|GetS_DockDoor) (select (Variables|Default|GetbStartOpen) (Variables|/Script/Engine.SceneComponent|GetRelativeLocation (Variables|Default|GetDoorPositionOpen)) (Variables|/Script/Engine.SceneComponent|GetRelativeLocation (Variables|Default|GetDoorPositionClosed))) false false)
  ;[1 1 1] Bind light to door
  (EventDispatchers|BindEventtoOnDoorOpened (delegate Custom|TurnDoorLightOn)))

(fn ConstructionScript
  (CallFunction|SetDockName)
  (CallFunction|UpdateDockScreenStatus))

(fn UpdateDockScreenStatus
  (bind _aswbp_crate_dock_screen (Utilities|Casting|CastToWBP_CrateDockScreen (UserInterface|GetWidget (Variables|Default|GetScreenWidget))))
  (bind _output_get (Variables|Default|SetDockScreenWidget _aswbp_crate_dock_screen))
  (Default|SetDockStatus _output_get (Variables|Default|GetDockStatus)))

(fn ReportDockingProgress
  (params (TimeLeft :type Float%20%28double-precision%29) (TimeTotal :type Float%20%28double-precision%29))
  (Default|SetDockingProgress (Variables|Default|GetDockScreenWidget) TimeLeft TimeTotal))

(fn SetDockStatus
  (params (NewStatus :type EDockStatus%20Enum :default "NewEnumerator0"))
  (Default|SetDockStatus (Variables|Default|GetDockScreenWidget) NewStatus)
  (Variables|Default|SetDockStatus NewStatus)
  (return))

(fn SetDockName
  (Default|SetDockName (Variables|Default|GetDockScreenWidget) (Variables|Default|GetDockName))
  (return))

(fn SetDockedCrateNumber
  (params (CrateNumber :type Text))
  (Default|SetDockedCrateNumber (Variables|Default|GetDockScreenWidget) CrateNumber))